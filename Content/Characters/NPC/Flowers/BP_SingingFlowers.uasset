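; BP_SingingFlowers is an NPC flower that sings while the player is inside its trigger.
; On overlap it pauses 2D music through GI_TMWR, then spawns and fades in the flower song at the flower's location.
; If a previous song component is still valid, it rechecks on a delay loop before spawning.
; On exit it resumes the music, then fades out and destroys the song component.
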(event `self.PlaySoundTrigger.OnComponentBeginOverlap`
  (params (OverlappedComponent :type "PrimitiveComponent Object Reference") (OtherActor :type "Actor Object Reference") (OtherComp :type "PrimitiveComponent Object Reference") (OtherBodyIndex :type Integer) (bFromSweep :type Boolean) (SweepResult :type "HitResult Structure (by ref)"))
  (if (`self.ActorHasTag` OtherActor "Player")
    (bind _asgi_tmwr (cast `/Game/Blueprints/GI_TMWR` (`GameplayStatics.GetGameInstance`)))
    (`/Game/Blueprints/GI_TMWR.PauseMusic2D` _asgi_tmwr true true)
    (`self.PlayingSong` :!label _label
      (:`then`
        (`KismetSystemLibrary.Delay` 5.0)
        (goto _label))
      (:`else`
        (bind _returnvalue (`GameplayStatics.SpawnSoundAtLocation` "/Game/Sound/Flowers/SC_FlowerSong.SC_FlowerSong" (`SceneComponent.K2_GetComponentLocation` (`self.Flower`)) (struct) 0.7 1.0 0.0 "/Game/Sound/DefaultAttenuation.DefaultAttenuation" null))
        (bind _output_get (set `self.PlayingSong` _returnvalue))
        (`AudioComponent.FadeIn` _output_get 2.0 0.7 0.0 "Linear")))))

(event `self.PlaySoundTrigger.OnComponentEndOverlap`
  (params (OverlappedComponent :type "PrimitiveComponent Object Reference") (OtherActor :type "Actor Object Reference") (OtherComp :type "PrimitiveComponent Object Reference") (OtherBodyIndex :type Integer))
  (if (`self.ActorHasTag` OtherActor "Player")
    (bind _asgi_tmwr (cast `/Game/Blueprints/GI_TMWR` (`GameplayStatics.GetGameInstance`)))
    (`/Game/Blueprints/GI_TMWR.PauseMusic2D` _asgi_tmwr true false)
    (bind _playingsong (`self.PlayingSong`)
      (:`then`
        (`AudioComponent.FadeOut` _playingsong 3.0 0.0 "Linear")
        (`KismetSystemLibrary.Delay` 3.0)
        (`ActorComponent.K2_DestroyComponent` (`self.PlayingSong`)))
      (:`else`))))

(fn `UserConstructionScript`)