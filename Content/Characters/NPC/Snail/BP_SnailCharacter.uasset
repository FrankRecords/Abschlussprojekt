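; BP_SnailCharacter is a quest-giver snail NPC that accepts mail from the player and moves off once its quest completes.
; Interacting while carrying mail removes a stacked envelope, reports the "returnmail" objective and turns in the "Snail" quest.
; It listens to the player quest log's completion event and, on a matching quest ID, chains AI MoveTo calls through its target points until the last one.
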(event `self.ReceiveBeginPlay`
  (add `/Game/Blueprints/QuestSystem/BPC_QuestLogComponent.OnQuestCompleted` (`self.GetComponentByClass` (`GameplayStatics.GetPlayerCharacter` 0) "/Game/Blueprints/QuestSystem/BPC_QuestLogComponent.BPC_QuestLogComponent_C") (delegate `SnailShouldMove`)))

(event `SnailShouldMove`
  (params (QuestActor :type "/Game/Blueprints/QuestSystem/BP_QuestBase Object Reference"))
  (if (== (`/Game/Blueprints/QuestSystem/BP_QuestBase.QuestID` QuestActor) (`.RowName` (break `DataTableRowHandle` (`/Game/Blueprints/QuestSystem/BPC_QuestGiverComponent.QuestData` (`self.BPC_QuestGiverComponent`)))))
    (`|AIMoveTo` self (`self.K2_GetActorLocation` (`|GetArrayItem` (`self.TargetPoints`) (`self.currentTarget`))) null 15.0 :!label _label
      (:`OnSuccess`
        (if (not (== (`self.currentTarget`) (- (`KismetArrayLibrary.Array_Length` (`self.TargetPoints`)) 1)))
          (set `self.currentTarget` (+ (`self.currentTarget`) 1))
          (goto _label))))))

(event `/Game/Blueprints/Interfaces/BPI_Interact.Interaction`
  (params (CharacterRef :type "/Game/Characters/ThirdPerson/Blueprints/BP_ThirdPersonCharacter Object Reference"))
  (if (`/Game/Characters/ThirdPerson/Blueprints/BP_ThirdPersonCharacter.HasMail?` CharacterRef)
    (bind _success_ (`/Game/CommonUI/03_Inventory/BP_Inventory.RemoveItem` (`/Game/Characters/ThirdPerson/Blueprints/BP_ThirdPersonCharacter.InventoryReference` CharacterRef) "/Game/CommonUI/03_Inventory/ItemClasses/SnailRiddle/BP_EquipItem_StackedEnvelopes.BP_EquipItem_StackedEnvelopes_C" 1))
    (if _success_
      (`/Game/Characters/ThirdPerson/Blueprints/BP_ThirdPersonCharacter.OnObjectiveIDCalled` CharacterRef "returnmail")
      (`/Game/Blueprints/QuestSystem/BPC_QuestLogComponent.TurnInQuest` (`/Game/Characters/ThirdPerson/Blueprints/BP_ThirdPersonCharacter.BPC_QuestLogComponent` CharacterRef) "Snail"))
    (else
      (`KismetSystemLibrary.PrintString` "NoMailYet"))))

(fn `InteractQuest`
  (returns (ObjectiveID :type String))
  (bind _objectiveid (`/Game/Blueprints/QuestSystem/BPC_QuestGiverComponent.InteractQuest` (`self.BPC_QuestGiverComponent`)))
  (return _objectiveid))

(fn `UserConstructionScript`)