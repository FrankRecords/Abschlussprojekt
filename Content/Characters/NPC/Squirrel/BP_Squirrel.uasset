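; BP_Squirrel is a squirrel NPC quest giver that reacts when the player completes a quest.
; On BeginPlay it binds to OnQuestCompleted on the player character's quest log component, without filtering on which quest finished.
; Completion loops the Happy_Idle animation and destroys the first BP_BlockWaySquirrel actor found in the level.
; InteractQuest forwards interaction to its quest giver component and returns the result.
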(event `self.ReceiveBeginPlay`
  (add `/Game/Blueprints/QuestSystem/BPC_QuestLogComponent.OnQuestCompleted` (`self.GetComponentByClass` (`GameplayStatics.GetPlayerCharacter` 0) "/Game/Blueprints/QuestSystem/BPC_QuestLogComponent.BPC_QuestLogComponent_C") (delegate `OnQuestCompleted`)))

(event `OnQuestCompleted`
  (params (QuestActor :type "/Game/Blueprints/QuestSystem/BP_QuestBase Object Reference"))
  (`SkeletalMeshComponent.PlayAnimation` (`self.Mesh`) "/Game/Characters/NPC/Squirrel/Anims/Happy_Idle.Happy_Idle" true)
  (bind _outactors (`GameplayStatics.GetAllActorsOfClass` "/Game/Blueprints/Actors/BP_BlockWaySquirrel.BP_BlockWaySquirrel_C"))
  (`self.K2_DestroyActor` (`|GetArrayItem` _outactors)))

(fn `InteractQuest`
  (returns (ObjectiveID :type String))
  (bind _objectiveid (`/Game/Blueprints/QuestSystem/BPC_QuestGiverComponent.InteractQuest` (`self.BPC_QuestGiverComponent`)))
  (return _objectiveid))

(fn `UserConstructionScript`)