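; BP_Friend is an NPC companion that appears when the player enters its trigger, speaks a dialogue and follows them.
; A timeline scales the initially zero-sized mesh up on entry and reverses it on exit.
; Only unplayed dialogues trigger the spawn, delayed sound and AIMoveTo chase, which reissues a second after each success or failure.
; The played-dialogue list persists through SaveData and LoadData, with loading requested from the GameInstance at BeginPlay.
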(event `self.ReceiveBeginPlay`
  (`SceneComponent.SetWorldScale3D` (`self.Mesh`) (0.0 0.0 0.0))
  (message `/Game/Blueprints/SaveGame/BPI_Persistence.RequestLoad` (`GameplayStatics.GetGameInstance`) self))

(event `self.TriggerFriend.OnComponentBeginOverlap`
  (params (OverlappedComponent :type "PrimitiveComponent Object Reference") (OtherActor :type "Actor Object Reference") (OtherComp :type "PrimitiveComponent Object Reference") (OtherBodyIndex :type Integer) (bFromSweep :type Boolean) (SweepResult :type "HitResult Structure (by ref)"))
  (if (`self.ActorHasTag` OtherActor "Player")
    (if (not (`KismetArrayLibrary.Array_Contains` (`self.PlayDialogues`) (`self.SoundToPlay`)))
      (`KismetArrayLibrary.Array_Add` (`self.PlayDialogues`) (`self.SoundToPlay`))
      (`self.SpawnFriend`)
      (`|ExecutionSequence`
        (:`then_0`
          (`KismetSystemLibrary.Delay` 1.0)
          (`GameplayStatics.SpawnSoundAttached` (`self.SoundToPlay`) (`self.Mesh`) "None" (0.0 0.0 0.0) (struct) "SnapToTarget" false 1.0 1.0 0.0 "/Game/Sound/FriendAttenuation.FriendAttenuation" null))
        (:`then_1`
          (set `CharacterMovementComponent.MaxWalkSpeed` (`self.FriendSpeed`) (`self.CharacterMovement`))
          (`|AIMoveTo` self (0.0 0.0 0.0) (`GameplayStatics.GetPlayerCharacter` 0) 150.0 :!label _label
            (:`OnSuccess`
              _)
            (:`OnFail`
              _))
          (`KismetSystemLibrary.Delay` 1.0)
          (goto _label))))))

(event `self.TriggerFriend.OnComponentEndOverlap`
  (params (OverlappedComponent :type "PrimitiveComponent Object Reference") (OtherActor :type "Actor Object Reference") (OtherComp :type "PrimitiveComponent Object Reference") (OtherBodyIndex :type Integer))
  (if (`self.ActorHasTag` OtherActor "Player")
    (`self.DespawnFriend`)))

(event `SpawnFriend`
  (bind (_direction _spawn) (`Timeline|SpawnFriendTimeline` :!label _label_2)
    (:`Update`
      (`SceneComponent.SetWorldScale3D` (`self.Mesh`) (`KismetMathLibrary.VLerp` (`self.StartScaleFriend`) (`self.EndScaleFriend`) _spawn)))))

(event `DespawnFriend`
  (goto _label_2 :!via `ReverseFromEnd`))

(event `/Game/Blueprints/SaveGame/BPI_Saveable.SaveData`
  (params (SaveGameRef :type "/Game/Blueprints/SaveGame/BP_SaveGame Object Reference"))
  (set `/Game/Blueprints/SaveGame/BP_SaveGame.PlayedDialogue` (`self.PlayDialogues`) SaveGameRef))

(event `/Game/Blueprints/SaveGame/BPI_Saveable.LoadData`
  (params (SaveGameRef :type "/Game/Blueprints/SaveGame/BP_SaveGame Object Reference"))
  (set `self.PlayDialogues` (`/Game/Blueprints/SaveGame/BP_SaveGame.PlayedDialogue` SaveGameRef)))

(fn `UserConstructionScript`)