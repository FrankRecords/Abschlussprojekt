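; BP_Friend_InventoryTut is a friend NPC that teaches the player to open the inventory.
; When the player enters its trigger, a not-yet-played dialogue is recorded, the friend spawns and walks to the player via AIMoveTo.
; In parallel it plays the attached voice line, then after its duration shows a tutorial hint widget with the OpenInventory input action and switches input to UI only.
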(event `self.TriggerFriend.OnComponentBeginOverlap`
  (params (OverlappedComponent :type "PrimitiveComponent Object Reference") (OtherActor :type "Actor Object Reference") (OtherComp :type "PrimitiveComponent Object Reference") (OtherBodyIndex :type Integer) (bFromSweep :type Boolean) (SweepResult :type "HitResult Structure (by ref)"))
  (bind _soundtoplay (`self.SoundToPlay`))
  (if (`self.ActorHasTag` OtherActor "Player")
    (if (not (`KismetArrayLibrary.Array_Contains` (`self.PlayDialogues`) (`self.SoundToPlay`)))
      (`KismetArrayLibrary.Array_Add` (`self.PlayDialogues`) (`self.SoundToPlay`))
      (`self.SpawnFriend`)
      (`|ExecutionSequence`
        (:`then_0`
          (`KismetSystemLibrary.Delay` 1.0)
          (`GameplayStatics.SpawnSoundAttached` _soundtoplay (`self.Mesh`) "None" (0.0 0.0 0.0) (struct) "SnapToTarget" false 1.0 1.0 0.0 "/Game/Sound/FriendAttenuation.FriendAttenuation" null)
          (`KismetSystemLibrary.Delay` (`SoundBase.Duration` _soundtoplay))
          (bind _returnvalue (`|CreateWidget` "/Game/CommonUI/11_Tutorial/UI_TutorialHint.UI_TutorialHint_C" null "to open the inventory" (make `DataTableRowHandle` "/Game/CommonUI/Foundation/Input/DT_InputAction.DT_InputAction" "OpenInventory") true))
          (`UserWidget.AddToViewport` _returnvalue 0)
          (`WidgetBlueprintLibrary.SetInputMode_UIOnlyEx` (`GameplayStatics.GetPlayerController` 0) _returnvalue))
        (:`then_1`
          (set `CharacterMovementComponent.MaxWalkSpeed` (`self.FriendSpeed`) (`self.CharacterMovement`))
          (`|AIMoveTo` self (0.0 0.0 0.0) (`GameplayStatics.GetPlayerCharacter` 0) 150.0
            (:`OnSuccess`
              _)
            (:`OnFail`
              _))
          (`KismetSystemLibrary.Delay` 1.0))))))

(fn `UserConstructionScript`
  (`parent.UserConstructionScript`))