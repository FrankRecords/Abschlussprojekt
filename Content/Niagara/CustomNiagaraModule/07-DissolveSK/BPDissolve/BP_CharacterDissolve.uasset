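; Character actor that, when something enters its trigger box, sends that actor a look-at message and dissolves after a short delay, once.
; A timeline drives the dissolve parameter on two dynamic Manny materials alongside an attached Niagara effect.
; A timer disables mesh collision, and the effect's finish optionally destroys the actor.
; A restore event reverses the dissolve and re-arms the trigger, but its end-overlap call is disconnected.
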(event `DissolveCharacter`
  (`|ExecutionSequence`
    (:`then_0`
      ;[1 1 1] Create Dynamic Materials
      (bind _returnvalue (`KismetMaterialLibrary.CreateDynamicMaterialInstance` "/Game/Niagara/CustomNiagaraModule/07-DissolveSK/BPDissolve/MI_Manny_01_BPDissolve.MI_Manny_01_BPDissolve"))
      (set `self.Created_Dyn_MI_Manny_01` _returnvalue)
      (bind _returnvalue_2 (`KismetMaterialLibrary.CreateDynamicMaterialInstance` "/Game/Niagara/CustomNiagaraModule/07-DissolveSK/BPDissolve/MI_Manny_02_BPDissolve.MI_Manny_02_BPDissolve"))
      (set `self.Created_Dyn_MI_Manny_02` _returnvalue_2))
    (:`then_1`
      ;[1 1 1] Setting Materials for Actor
      (`PrimitiveComponent.SetMaterial` (`self.SkeletalMesh`) 0 (`self.Created_Dyn_MI_Manny_01`))
      (`PrimitiveComponent.SetMaterial` (`self.SkeletalMesh`) 1 (`self.Created_Dyn_MI_Manny_02`)))
    (:`then_2`
      ;[1 0.7987 0] Timeline for dissolving Materials
      (bind (_direction _dissolvetrack) (`Timeline|DissolveTimeline` :!via `PlayFromStart` :!label _label)
        (:`Update`
          (`MaterialInstanceDynamic.SetScalarParameterValue` (`self.Created_Dyn_MI_Manny_01`) "DissolveAmount" _dissolvetrack)
          (`MaterialInstanceDynamic.SetScalarParameterValue` (`self.Created_Dyn_MI_Manny_02`) "DissolveAmount" _dissolvetrack))))
    (:`then_3`
      ;[1 0.3758 0] Spawn Niagara VFX
      (bind _returnvalue_3 (`NiagaraFunctionLibrary.SpawnSystemAttached` "/Game/Niagara/CustomNiagaraModule/07-DissolveSK/NS_BPDissolve.NS_BPDissolve" (`self.SkeletalMesh`) "None" (0.0 0.0 0.0) (struct) "SnapToTarget"))
      (add `NiagaraComponent.OnSystemFinished` _returnvalue_3 (delegate `DestroyActor`)))
    (:`then_4`
      ;[0.6195 0 1] Collision Timer Event
      (bind _returnvalue_4 (`KismetSystemLibrary.K2_SetTimerDelegate` (delegate `SetCollisionDisabled`) 2.0 false true))
      (set `self.CollisionTimer` _returnvalue_4))))

(event `RestoreCharacter`
  ;[0 0.5823 1] Restoring character
  (`|ExecutionSequence`
    (:`then_0`
      (`KismetSystemLibrary.K2_ClearAndInvalidateTimerHandle` (`self.CollisionTimer`))
      (`PrimitiveComponent.SetCollisionEnabled` (`self.SkeletalMesh`) "QueryAndPhysics")
      (goto _label :!via `Reverse`))
    (:`then_1`
      (goto _label_2 :!via `Reset`))))

(event `DestroyActor`
  (params (PSystem :type "NiagaraComponent Object Reference"))
  (if (`self.DestroyAfterLookAt`)
    (`self.K2_DestroyActor`)))

(event `SetCollisionDisabled`
  ;[0.6195 0 1] Collision Timer Event
  (`PrimitiveComponent.SetCollisionEnabled` (`self.SkeletalMesh`) "NoCollision"))

(event `self.Box.OnComponentBeginOverlap`
  (params (OverlappedComponent :type "PrimitiveComponent Object Reference") (OtherActor :type "Actor Object Reference") (OtherComp :type "PrimitiveComponent Object Reference") (OtherBodyIndex :type Integer) (bFromSweep :type Boolean) (SweepResult :type "HitResult Structure (by ref)"))
  (`/Engine/EditorBlueprintResources/StandardMacros.DoOnce` false :!label _label_2
    (:`Completed`
      (message `/Game/Blueprints/Interfaces/BPI_LookAt.LookAt` OtherActor (`self.Arrow`))
      (`KismetSystemLibrary.Delay` 1.0)
      (`self.DissolveCharacter`))))

(event `self.Box.OnComponentEndOverlap`
  (params (OverlappedComponent :type "PrimitiveComponent Object Reference") (OtherActor :type "Actor Object Reference") (OtherComp :type "PrimitiveComponent Object Reference") (OtherBodyIndex :type Integer)))

(fn `UserConstructionScript`
  (`SceneComponent.K2_SetRelativeTransform` (`self.Box`) (`self.CollisionTransform`) false false))