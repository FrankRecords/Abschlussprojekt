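; BP_TextureBaker is an editor utility Blueprint that bakes a material's output into a static texture asset.
; Its BakeTexture function checks that the render target and source material are valid, then draws the material into the render target.
; It saves that result as a Texture2D named TextureFromRenderTarget through an editor-only node.
; The event graph and construction script are empty, so nothing runs automatically.
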(fn `BakeTexture`
  (if (and (`KismetSystemLibrary.IsValid` (`self.RenderTargetToDraw`)) (`KismetSystemLibrary.IsValid` (`self.MaterialToDrawFrom`)))
    (`KismetRenderingLibrary.DrawMaterialToRenderTarget` (`self.RenderTargetToDraw`) (`self.MaterialToDrawFrom`))
    (`KismetRenderingLibrary.RenderTargetCreateStaticTexture2DEditorOnly` (`self.RenderTargetToDraw`) "TextureFromRenderTarget")))

(fn `UserConstructionScript`)