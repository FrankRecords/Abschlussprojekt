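; Spawner actor that repeatedly launches BP_ProjectileMaster projectiles to play configurable Niagara projectile effects.
; On BeginPlay it fires once, then a looping timer respawns at the set gap from the actor's location.
; Each projectile receives muzzle, main and hit impact effects, spawn offset, destroy delay and a decoration particle loop duration.
; Velocity is set along a fixed X vector scaled by projectile speed, independent of the spawner's rotation.
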(event `self.ReceiveBeginPlay`
  (`self.SpawnProjectileVFX`)
  (`KismetSystemLibrary.K2_SetTimerDelegate` (delegate `SpawnProjectileVFX`) (`self.ProjectileSpawnGap`) true))

(event `SpawnProjectileVFX`
  (bind _returnvalue (`|SpawnActorFromClass` "/Game/Niagara/VFXSpawner/BP_ProjectileMaster.BP_ProjectileMaster_C" (`KismetMathLibrary.MakeTransform` (`self.K2_GetActorLocation`)) "Undefined" "MultiplyWithRoot" null null))
  (bind _output_get (set `self.SpawnedProjectile` _returnvalue))
  (`/Engine/EditorBlueprintResources/StandardMacros.IsValid` _output_get
    (:`Is Valid`
      (`|ExecutionSequence`
        (:`then_0`
          ;[1 1 1] Setting VFX Niagara Variables
          (set `/Game/Niagara/VFXSpawner/BP_ProjectileMaster.MuzzleVFX` (`self.Muzzle VFX`) (`self.SpawnedProjectile`))
          (`NiagaraComponent.SetAsset` (`/Game/Niagara/VFXSpawner/BP_ProjectileMaster.ProjectileVFXComponent` (`self.SpawnedProjectile`)) (`self.MainProjectileVFX`) true)
          (set `/Game/Niagara/VFXSpawner/BP_ProjectileMaster.HitImpactVFX` (`self.Hit Impact VFX`) (`self.SpawnedProjectile`)))
        (:`then_1`
          ;[1 1 1] Setting projectile speed
          (set `MovementComponent.Velocity` (* (`self.ProjectileSpeed`) (1.0 0.0 0.0)) (`/Game/Niagara/VFXSpawner/BP_ProjectileMaster.ProjectileVFXMovementComp` (`self.SpawnedProjectile`))))
        (:`then_2`
          (set `/Game/Niagara/VFXSpawner/BP_ProjectileMaster.MuzzleHitImpactSpawnOffset` (`self.Muzzle Hit Impact Spawn Offset`) (`self.SpawnedProjectile`))
          (set `/Game/Niagara/VFXSpawner/BP_ProjectileMaster.ProjectileDestroyDelay` (`self.Projectile Destroy Delay`) (`self.SpawnedProjectile`))
          (`NiagaraComponent.SetVariableFloat` (`/Game/Niagara/VFXSpawner/BP_ProjectileMaster.ProjectileVFXComponent` (`self.SpawnedProjectile`)) "DecorationParticlesLoopDuration" (`self.DecorationParticlesLoopDuration`)))))))

(fn `UserConstructionScript`)