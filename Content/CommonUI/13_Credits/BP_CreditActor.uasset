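; BP_CreditActor runs the credits sequence, playing the Credits_TMWR media source and showing the WBP_Credits widget.
; On BeginPlay it adds the widget, starts the media player and enables input in Game and UI mode, returning to L_Menu when playback ends.
; A hold-to-skip on IA_UI_SkipCutscene uses a Timeline to drive the widget's slider, loading L_Menu when it finishes and resetting when the input completes.
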(event `self.ReceiveBeginPlay`
  (bind _returnvalue (`GameplayStatics.GetPlayerController` 0))
  (add `MediaPlayer.OnEndReached` (`self.MediaPlayer`) (delegate `ReturnToMainMenu`))
  (bind _returnvalue_2 (`|CreateWidget` "/Game/CommonUI/13_Credits/WBP_Credits.WBP_Credits_C" (`GameplayStatics.GetPlayerController` 0)))
  (set `self.CreditsWidget` _returnvalue_2)
  (`UserWidget.AddToViewport` (`self.CreditsWidget`) 0)
  (`MediaPlayer.OpenSource` (`self.MediaPlayer`) "/Game/Movies/Credits_TMWR.Credits_TMWR")
  (`self.EnableInput` _returnvalue)
  (`WidgetBlueprintLibrary.SetInputMode_GameAndUIEx` _returnvalue _returnvalue_2))

(event `ReturnToMainMenu`
  (`GameplayStatics.OpenLevelBySoftObjectPtr` "/Game/Levels/L_Menu.L_Menu"))

(event `EnhancedInput|/Game/CommonUI/Foundation/Input/EnhancedInput/Actions/IA_UI_SkipCutscene`
  (params (ActionValue :type Boolean) (ElapsedSeconds :type "Float (double-precision)") (TriggeredSeconds :type "Float (double-precision)") (InputAction :type "InputAction Object Reference" :default "/Game/CommonUI/Foundation/Input/EnhancedInput/Actions/IA_UI_SkipCutscene.IA_UI_SkipCutscene"))
  (:`Triggered`
    (if (`Widget.IsInViewport` (`self.CreditsWidget`))
      (bind (_direction _time) (`Timeline|Timeline` :!via `PlayFromStart` :!label _label)
        (:`Update`
          (`/Game/CommonUI/13_Credits/WBP_Credits.UpdateSliderValue` (`self.CreditsWidget`) _time))
        (:`Finished`
          (`GameplayStatics.OpenLevelBySoftObjectPtr` "/Game/Levels/L_Menu.L_Menu")))))
  (:`Completed`
    (`|ExecutionSequence`
      (:`then_0`
        (goto _label :!via `Stop`))
      (:`then_1`
        (`/Game/CommonUI/13_Credits/WBP_Credits.UpdateSliderValue` (`self.CreditsWidget`) 0.0)))))

(fn `UserConstructionScript`)