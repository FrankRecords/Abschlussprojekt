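; Pickup item actor that gives a set amount of an item class to a character's inventory when that character interacts with it.
; The Interaction event calls AddItem on the character's inventory, keeping any leftover amount for later or destroying the actor once everything is taken.
; The sphere overlap event is empty, and a duplicate pickup path that casts to BP_ThirdPersonCharacter is left unconnected.
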(event `self.Sphere.OnComponentBeginOverlap`
  (params (OverlappedComponent :type "PrimitiveComponent Object Reference") (OtherActor :type "Actor Object Reference") (OtherComp :type "PrimitiveComponent Object Reference") (OtherBodyIndex :type Integer) (bFromSweep :type Boolean) (SweepResult :type "HitResult Structure (by ref)")))

(event `/Game/Blueprints/Interfaces/BPI_Interact.Interaction`
  (params (CharacterRef :type "/Game/Characters/ThirdPerson/Blueprints/BP_ThirdPersonCharacter Object Reference"))
  (bind _inventoryreference (`/Game/Characters/ThirdPerson/Blueprints/BP_ThirdPersonCharacter.InventoryReference` CharacterRef))
  (`/Engine/EditorBlueprintResources/StandardMacros.IsValid` _inventoryreference
    (:`Is Valid`
      (bind (_success_ _restamount) (`/Game/CommonUI/Inventory/BP_Inventory.AddItem` _inventoryreference (`self.ItemToAdd`) (`self.AmountToAdd`)))
      (if _success_
        (if (> _restamount 0)
          (set `self.AmountToAdd` _restamount)
          (else
            (`self.K2_DestroyActor`)))))))

(fn `UserConstructionScript`)