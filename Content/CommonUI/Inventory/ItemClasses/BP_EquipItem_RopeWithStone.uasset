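; BP_EquipItem_RopeWithStone is an inventory item actor: a rope with a stone that can be picked up.
; On BeginPlay it enables physics on StoneStart and Rope, attaches the rope's end to the Stone component and sets its own class as the item to add.
; Interaction adds the item to the character's inventory, then keeps any leftover amount or destroys the actor when none remains.
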(event `self.ReceiveBeginPlay`
  (`PrimitiveComponent.SetSimulatePhysics` (`self.StoneStart`) true)
  (`PrimitiveComponent.SetSimulatePhysics` (`self.Rope`) true)
  (`CableComponent.SetAttachEndToComponent` (`self.Rope`) (`self.Stone`) "None")
  (set `self.ItemToAdd` "BP_EquipItem_RopeWithStone_C"))

(event `/Game/Blueprints/Interfaces/BPI_Interact.Interaction`
  (params (CharacterRef :type "/Game/Characters/ThirdPerson/Blueprints/BP_ThirdPersonCharacter Object Reference"))
  (bind _inventoryreference (`/Game/Characters/ThirdPerson/Blueprints/BP_ThirdPersonCharacter.InventoryReference` CharacterRef))
  (`/Engine/EditorBlueprintResources/StandardMacros.IsValid` _inventoryreference
    (:`Is Valid`
      (bind (_success_ _restamount) (`/Game/CommonUI/Inventory/BP_Inventory.AddItem` _inventoryreference (`self.ItemToAdd`) (`self.AmountToAdd`)))
      (if _success_
        (if (> _restamount 0)
          (set `self.AmountToAdd` _restamount)
          (else
            (`self.K2_DestroyActor`)))))))

(fn `UserConstructionScript`
  (`parent.UserConstructionScript`))