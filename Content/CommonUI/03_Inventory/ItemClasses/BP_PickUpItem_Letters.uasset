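; BP_PickUpItem_Letters is a pickup item, apparently the letters tied to the "Snail" quest, that removes itself once that quest is taken or finished.
; On BeginPlay it runs the parent logic, then gets the player's BP_ThirdPersonCharacter and reads its BPCQuestLogComponent.
; It loops over the completed and current active quest lists and destroys the actor if "Snail" appears in either.
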(event `self.ReceiveBeginPlay`
  (`parent.ReceiveBeginPlay`)
  (bind _asbp_third_person_character (cast `/Game/Characters/ThirdPerson/Blueprints/BP_ThirdPersonCharacter` (`GameplayStatics.GetPlayerCharacter` 0)))
  (bind _bpc_questlogcomponent (`/Game/Characters/ThirdPerson/Blueprints/BP_ThirdPersonCharacter.BPC_QuestLogComponent` _asbp_third_person_character))
  (for _array_element (`/Game/Blueprints/QuestSystem/BPC_QuestLogComponent.CompletedQuests` _bpc_questlogcomponent)
    (if (== _array_element "Snail")
      (`self.K2_DestroyActor` :!label _label)))
  (for _array_element_2 (`/Game/Blueprints/QuestSystem/BPC_QuestLogComponent.CurrentActiveQuests` _bpc_questlogcomponent)
    (if (== _array_element_2 "Snail")
      (goto _label))))

(fn `UserConstructionScript`
  (`parent.UserConstructionScript`))