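; World pickup actor that gives an item to the player's inventory, gated on its quest being active.
; Construction and BeginPlay take the mesh from the equip item's class defaults.
; Sphere overlaps toggle the outline and pickup prompt for the third-person character.
; A successful Interaction requests a save message, plays backpack animation and sound, then either keeps the leftover amount or reports the objective ID and destroys itself.
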(event `self.ReceiveBeginPlay`
  (bind _itemtoadd (`self.ItemToAdd`))
  (set `self.PlayerRef` (`/Game/Blueprints/QuestSystem/CommonFunctionLibrary.GetMyPlayerCharacter`))
  (if (`.HasStaticMesh_27_C8D0906E4966653EA5402BA4D2EB87A1` (break `/Game/CommonUI/03_Inventory/Inventory_Structure/S_ItemInfo` (`.ItemInfo` (defaults `Object` _itemtoadd))))
    (bind _asbp_equip_item_master (castclass `/Game/CommonUI/03_Inventory/ItemClasses/BP_EquipItemMaster` _itemtoadd))
    (`StaticMeshComponent.SetStaticMesh` (`self.StaticMesh`) (`.EquipStaticMesh` (defaults `Object` _asbp_equip_item_master)))))

(event `/Game/Blueprints/Interfaces/BPI_Interact.Interaction`
  (params (CharacterRef :type "/Game/Characters/ThirdPerson/Blueprints/BP_ThirdPersonCharacter Object Reference"))
  (bind _inventoryreference (`/Game/Characters/ThirdPerson/Blueprints/BP_ThirdPersonCharacter.InventoryReference` CharacterRef))
  (`/Engine/EditorBlueprintResources/StandardMacros.IsValid` _inventoryreference
    (:`Is Valid`
      (bind _active_ (`/Game/Blueprints/QuestSystem/BPC_QuestLogComponent.IsActiveQuest` (`/Game/Characters/ThirdPerson/Blueprints/BP_ThirdPersonCharacter.BPC_QuestLogComponent` (`self.PlayerRef`)) (`self.Quest ID`)))
      (if _active_
        (bind (_success_ _restamount) (`/Game/CommonUI/03_Inventory/BP_Inventory.AddItem` _inventoryreference (`self.ItemToAdd`) (`self.AmountToAdd`)))
        (if _success_
          (message `/Game/Blueprints/SaveGame/BPI_Persistence.RequestSave` (`GameplayStatics.GetGameInstance`) true "SaveSlot1")
          (`SkeletalMeshComponent.PlayAnimation` (`/Game/Characters/ThirdPerson/Blueprints/BP_ThirdPersonCharacter.Backpack` (`/Game/CommonUI/03_Inventory/BP_Inventory.TPCharRef` _inventoryreference)) "/Game/Assets/Backpack/RiggedBackpack/AdventureBackpack/Animations/Animation_Anim_PickupItem.Animation_Anim_PickupItem" false)
          (`GameplayStatics.PlaySound2D` "/Game/CommonUI/01_AudioUI/Inventory/Whoosh_Source_Cloth_Backpack_02.Whoosh_Source_Cloth_Backpack_02" 0.5 1.0 0.0 null null)
          (if (> _restamount 0)
            (set `self.AmountToAdd` _restamount)
            (else
              (`/Game/Characters/ThirdPerson/Blueprints/BP_ThirdPersonCharacter.OnObjectiveIDCalled` (`/Game/Blueprints/QuestSystem/CommonFunctionLibrary.GetMyPlayerCharacter`) (`self.Objective ID`))
              (`self.K2_DestroyActor`))))))))

(event `self.Sphere.OnComponentBeginOverlap`
  (params (OverlappedComponent :type "PrimitiveComponent Object Reference") (OtherActor :type "Actor Object Reference") (OtherComp :type "PrimitiveComponent Object Reference") (OtherBodyIndex :type Integer) (bFromSweep :type Boolean) (SweepResult :type "HitResult Structure (by ref)"))
  (bind _asbp_third_person_character (cast `/Game/Characters/ThirdPerson/Blueprints/BP_ThirdPersonCharacter` OtherActor))
  (bind _ac_outliner_advanced (`/Game/Characters/ThirdPerson/Blueprints/BP_ThirdPersonCharacter.AC_Outliner_Advanced` _asbp_third_person_character))
  (`/Game/Hyper/Core/Outliner_System/Blueprints/AC_Outliner_Abstract.Client: Switch Outline on actor` _ac_outliner_advanced self "NewEnumerator0" (not (`/Game/Hyper/Core/Outliner_System/Blueprints/AC_Outliner_Abstract.Check if actor has outliner` _ac_outliner_advanced self)) "NewEnumerator0")
  (`SceneComponent.SetVisibility` (`self.PickupWidget`) true false))

(event `self.Sphere.OnComponentEndOverlap`
  (params (OverlappedComponent :type "PrimitiveComponent Object Reference") (OtherActor :type "Actor Object Reference") (OtherComp :type "PrimitiveComponent Object Reference") (OtherBodyIndex :type Integer))
  (bind _asbp_third_person_character (cast `/Game/Characters/ThirdPerson/Blueprints/BP_ThirdPersonCharacter` OtherActor))
  (bind _ac_outliner_advanced (`/Game/Characters/ThirdPerson/Blueprints/BP_ThirdPersonCharacter.AC_Outliner_Advanced` _asbp_third_person_character))
  (`/Game/Hyper/Core/Outliner_System/Blueprints/AC_Outliner_Abstract.Client: Switch Outline on actor` _ac_outliner_advanced self "NewEnumerator0" (not (`/Game/Hyper/Core/Outliner_System/Blueprints/AC_Outliner_Abstract.Check if actor has outliner` _ac_outliner_advanced self)) "NewEnumerator0")
  (`SceneComponent.SetVisibility` (`self.PickupWidget`) false false))

(fn `UserConstructionScript`
  (bind _itemtoadd (`self.ItemToAdd`))
  (if (`.HasStaticMesh_27_C8D0906E4966653EA5402BA4D2EB87A1` (break `/Game/CommonUI/03_Inventory/Inventory_Structure/S_ItemInfo` (`.ItemInfo` (defaults `Object` _itemtoadd))))
    (bind _asbp_equip_item_master (castclass `/Game/CommonUI/03_Inventory/ItemClasses/BP_EquipItemMaster` _itemtoadd))
    (`StaticMeshComponent.SetStaticMesh` (`self.StaticMesh`) (`.EquipStaticMesh` (defaults `Object` _asbp_equip_item_master)))))