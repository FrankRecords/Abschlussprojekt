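; Master Blueprint for equippable inventory items, handling equipping and throwing.
; On use, it passes itself to the character's EquipItem and destroys itself if that returns false.
; ThrowItem spawns the given class at the character's ThrowRef, adding a physics mesh at runtime and launching it with the throw velocity.
; RopeWithStone is special-cased: its existing Stone component is launched, and no inventory reference is passed.
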(event `self.EventOnUsed`
  (bind _success_ (`/Game/Characters/ThirdPerson/Blueprints/BP_ThirdPersonCharacter.EquipItem` (`/Game/CommonUI/03_Inventory/BP_Inventory.TPCharRef` (`self.Inventory`)) self))
  (if (not _success_)
    (`self.K2_DestroyActor`)))

(event `ThrowItem`
  (params (ThrowVelocity :type "Vector Structure") (CharacterRef :type "/Game/Characters/ThirdPerson/Blueprints/BP_ThirdPersonCharacter Object Reference") (ClassToSpawn :type "/Game/CommonUI/03_Inventory/ItemClasses/BP_MasterItem Class Reference") (MeshToSpawn :type "StaticMesh Object Reference"))
  (bind _returnvalue (`SceneComponent.K2_GetComponentLocation` (`/Game/Characters/ThirdPerson/Blueprints/BP_ThirdPersonCharacter.ThrowRef` CharacterRef)))
  (if (not (== ClassToSpawn "/Game/CommonUI/03_Inventory/ItemClasses/BP_EquipItem_RopeWithStone.BP_EquipItem_RopeWithStone_C"))
    (bind _returnvalue_2 (`|SpawnActorFromClass` ClassToSpawn (`KismetMathLibrary.MakeTransform` _returnvalue (struct) (0.25 0.25 0.25)) "AlwaysSpawn" "MultiplyWithRoot" null (`/Game/Characters/ThirdPerson/Blueprints/BP_ThirdPersonCharacter.InventoryReference` CharacterRef) 0 (struct) null))
    (bind _returnvalue_3 (`AddComponent|NODE_AddStaticMeshComponent-0` :`self` _returnvalue_2))
    (`StaticMeshComponent.SetStaticMesh` _returnvalue_3 MeshToSpawn)
    (`PrimitiveComponent.SetCollisionEnabled` _returnvalue_3 "QueryAndPhysics")
    (`PrimitiveComponent.SetSimulatePhysics` _returnvalue_3 true)
    (`PrimitiveComponent.SetAllPhysicsLinearVelocity` _returnvalue_3 ThrowVelocity false)
    (else
      (bind _returnvalue_4 (`|SpawnActorFromClass` "/Game/CommonUI/03_Inventory/ItemClasses/BP_EquipItem_RopeWithStone.BP_EquipItem_RopeWithStone_C" (`KismetMathLibrary.MakeTransform` _returnvalue (struct) (0.25 0.25 0.25)) "AlwaysSpawn" "MultiplyWithRoot" null null 0 (struct) null))
      (bind _stone (`/Game/CommonUI/03_Inventory/ItemClasses/BP_EquipItem_RopeWithStone.Stone` _returnvalue_4))
      (`PrimitiveComponent.SetCollisionEnabled` _stone "QueryAndPhysics")
      (`PrimitiveComponent.SetSimulatePhysics` _stone true)
      (`PrimitiveComponent.SetAllPhysicsLinearVelocity` _stone ThrowVelocity false))))

(fn `UserConstructionScript`
  (`parent.UserConstructionScript`))