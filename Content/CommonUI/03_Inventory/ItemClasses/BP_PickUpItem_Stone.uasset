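; Stone pickup item that the player collects into the inventory as part of a quest.
; Interaction only works once the character's TriedKnive flag is set, the inventory is valid and the pickup's quest is active.
; A successful add requests an async save and plays the backpack pickup animation and sound.
; If nothing is left over, it reports the quest objective through the player character and destroys itself.
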(event `/Game/Blueprints/Interfaces/BPI_Interact.Interaction`
  (params (CharacterRef :type "/Game/Characters/ThirdPerson/Blueprints/BP_ThirdPersonCharacter Object Reference"))
  (bind _inventoryreference (`/Game/Characters/ThirdPerson/Blueprints/BP_ThirdPersonCharacter.InventoryReference` CharacterRef))
  (if (`/Game/Characters/ThirdPerson/Blueprints/BP_ThirdPersonCharacter.TriedKnive?` CharacterRef)
    (`/Engine/EditorBlueprintResources/StandardMacros.IsValid` _inventoryreference
      (:`Is Valid`
        (bind _active_ (`/Game/Blueprints/QuestSystem/BPC_QuestLogComponent.IsActiveQuest` (`/Game/Characters/ThirdPerson/Blueprints/BP_ThirdPersonCharacter.BPC_QuestLogComponent` (`self.PlayerRef`)) (`self.Quest ID`)))
        (if _active_
          (bind (_success_ _restamount) (`/Game/CommonUI/03_Inventory/BP_Inventory.AddItem` _inventoryreference (`self.ItemToAdd`) (`self.AmountToAdd`)))
          (if _success_
            (message `/Game/Blueprints/SaveGame/BPI_Persistence.RequestSave` (`GameplayStatics.GetGameInstance`) true "SaveSlot1")
            (`SkeletalMeshComponent.PlayAnimation` (`/Game/Characters/ThirdPerson/Blueprints/BP_ThirdPersonCharacter.Backpack` (`/Game/CommonUI/03_Inventory/BP_Inventory.TPCharRef` _inventoryreference)) "/Game/Assets/Backpack/RiggedBackpack/AdventureBackpack/Animations/Animation_Anim_PickupItem.Animation_Anim_PickupItem" false)
            (`GameplayStatics.PlaySound2D` "/Game/CommonUI/01_AudioUI/Inventory/Whoosh_Source_Cloth_Backpack_02.Whoosh_Source_Cloth_Backpack_02" 0.5 1.0 0.0 null null)
            (if (not (> _restamount 0))
              (`/Game/Characters/ThirdPerson/Blueprints/BP_ThirdPersonCharacter.OnObjectiveIDCalled` (`/Game/Blueprints/QuestSystem/CommonFunctionLibrary.GetMyPlayerCharacter`) (`self.Objective ID`))
              (`self.K2_DestroyActor`))))))))

(fn `UserConstructionScript`
  (`parent.UserConstructionScript`))