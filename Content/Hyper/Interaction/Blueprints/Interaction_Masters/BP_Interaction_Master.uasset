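; BP_Interaction_Master is a base interaction trigger, such as a switch, that drives target actors through Interact and Toggle messages.
; ExecuteTriggers runs three optional modes: activate regardless of state, match targets to TriggerIsDown, or toggle opposing On/Off lists for puzzle logic.
; The construction script seeds TriggerIsDown from TriggerStartsDown.
; BeginPlay, on authority only, applies both state-based modes to set initial target states.
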(event `Execute Triggers`
  (params (`Owning Controller` :type "Controller Object Reference"))
  (bind _targets_to_activate (`self.Targets to activate`))
  (bind _targets_to_activate_2 (`self.Targets to activate`))
  (`|ExecutionSequence`
    (:`then_0`
      ;[0.05127 0.05127 0.05127] Activates target actors regardsless of state. E.g. if something is on, it will be off. Or of something is off, it will be on. This does not force any state.
      (if (`self.Activate target actors regardless of state`)
        (if (`KismetArrayLibrary.Array_IsNotEmpty` _targets_to_activate)
          (message `/Game/Hyper/Core/Interaction/Interfaces/BPI_Interact.Interact` _targets_to_activate `Owning Controller`))))
    (:`then_1`
      ;[0.05127 0.05127 0.05127] When switch is down, Turn ON
      ; When switch is UP, Turn OFF
      (if (`self.Turn off when switch is down`) :!label _label
        (if (`self.Trigger is down`)
          (message `/Game/Hyper/Core/Interaction/Interfaces/BPI_Toggle.Toggle` _targets_to_activate_2 true `Owning Controller`)
          (else
            (message `/Game/Hyper/Core/Interaction/Interfaces/BPI_Toggle.Toggle` _targets_to_activate_2 false `Owning Controller`)))))
    (:`then_2`
      ;[0.05127 0.05127 0.05127] Custom toggle overrides the ON list to on when the switch is down and the OFF list to off.
      ; If the switch is up, it reverses. So the whole ON list is off, and Off list goes ON.
      ; This can be usefull to make puzzle logic
      (if (`self.Use Custom Toggle`) :!label _label_2
        (if (`self.Trigger is down`)
          (message `/Game/Hyper/Core/Interaction/Interfaces/BPI_Toggle.Toggle` (`self.Targets to toggle On`) true `Owning Controller`)
          (message `/Game/Hyper/Core/Interaction/Interfaces/BPI_Toggle.Toggle` (`self.Targets to toggle Off`) false `Owning Controller`)
          (else
            (message `/Game/Hyper/Core/Interaction/Interfaces/BPI_Toggle.Toggle` (`self.Targets to toggle On`) false `Owning Controller`)
            (message `/Game/Hyper/Core/Interaction/Interfaces/BPI_Toggle.Toggle` (`self.Targets to toggle Off`) true `Owning Controller`)))))))

(event `self.ReceiveBeginPlay`
  ;[0.05127 0.05127 0.05127] Make sure to set the initial logic if using a custom toggle
  (`/Engine/EditorBlueprintResources/ActorMacros.Switch Has Authority`
    (:`Authority`
      (if (or (`self.Use Custom Toggle`) (`self.Turn off when switch is down`))
        (`|ExecutionSequence`
          (:`then_0`
            (goto _label))
          (:`then_1`
            (goto _label_2)))))))

(fn `UserConstructionScript`
  (set `self.Trigger is down` (`self.Trigger Starts Down`)))