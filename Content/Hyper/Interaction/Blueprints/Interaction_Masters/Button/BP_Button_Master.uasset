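; Master interaction button Blueprint that animates a press and executes its triggers, fired by trigger-box overlap or button events.
; The Press timeline drives the button's height and emissive color through a dynamic material created in the construction script.
; An overlap count holds the button down while actors remain.
; Clickable buttons auto-release after firing; others stay down until released and fire triggers on both press and release.
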(event `Trigger Button Down`
  (params (`Owning Controller` :type "Controller Object Reference"))
  ;[0.05098 0.05098 0.05098] Checking the current overlapping actors and not deactivating when there is still a character in the trigger box.
  (set `self.Overlapping Actors` (+ (`self.Overlapping Actors`) 1))
  (bind (_direction _press _glow) (`Timeline|Press` :!label _label) ; Timeline for animating the button press
    (:`Update`
      (`self.Set Button Position and Color` _press _glow))
    (:`Finished`
      (bind _returnvalue (`|EnumEquality` _direction "Forward"))
      ;[0.05127 0.05127 0.05127] When timeline is finished, the switch is down and execture the triggers
      (if (not (and _returnvalue (`self.Trigger is down`)))
        (bind _output_get (set `self.Trigger is down` _returnvalue))
        (if _output_get
          ;[0.05127 0.05127 0.05127] If the button is a clickable button. The button returns back to the original state after triggered. If this is not true, it will be a button which is not returning automaticly but should be done by event.
          (if (`self.Is Clickable Button`)
            (`self.Trigger Button Up`))
          (`self.Execute Triggers` `Owning Controller` :!label _label_2)
          (elif (not (`self.Is Clickable Button`))
            (goto _label_2)))))))

(event `self.Trigger.OnComponentBeginOverlap`
  (params (OverlappedComponent :type "PrimitiveComponent Object Reference") (OtherActor :type "Actor Object Reference") (OtherComp :type "PrimitiveComponent Object Reference") (OtherBodyIndex :type Integer) (bFromSweep :type Boolean) (SweepResult :type "HitResult Structure (by ref)"))
  ;[0.05127 0.05127 0.05127] Use trigger to activate button. On overlap it will be excecuted
  (if (`self.Use Triggerbox to excecute button`)
    (`self.Trigger Button Down` (`self.GetInstigatorController` OtherActor))))

(event `Trigger Button Up`
  ;[0.05098 0.05098 0.05098] Checking the current overlapping actors and not deactivating when there is still a character in the trigger box.
  (if (`self.Trigger is down`)
    (bind _output_get (set `self.Overlapping Actors` (- (`self.Overlapping Actors`) 1)))
    (if (<= _output_get 0)
      (goto _label :!via `Reverse`))))

(event `self.Trigger.OnComponentEndOverlap`
  (params (OverlappedComponent :type "PrimitiveComponent Object Reference") (OtherActor :type "Actor Object Reference") (OtherComp :type "PrimitiveComponent Object Reference") (OtherBodyIndex :type Integer))
  ;[0.05127 0.05127 0.05127] Use trigger to activate button. On overlap it will be excecuted
  (if (`self.Use Triggerbox to excecute button`)
    (`self.Trigger Button Up`)))

(fn `Set Button Position and Color`
  (params (Position :type "Float (double-precision)") (`Alpha Color` :type "Float (single-precision)"))
  (`SceneComponent.K2_SetRelativeLocation` (`self.Button`) (`KismetMathLibrary.MakeVector` 0.0 0.0 (* Position (`self.Press Range`))) false false) ; Move button up/down
  ;[0.05127 0.05127 0.05127] Set color when pressed
  (`MaterialInstanceDynamic.SetVectorParameterValue` (`self.Button material`) (`self.Pressed Color Parameter Value`) (`KismetMathLibrary.LinearColorLerp` (select `bool` (`self.Emissive when not pressed?`) :`true` (`self.Button_Color`)) (`self.Pressed_Color`) (`local.Alpha Color`))) ; Change emissive color of the button
)

(fn `UserConstructionScript`
  (`parent.UserConstructionScript`)
  (`StaticMeshComponent.SetStaticMesh` (`self.Button base`) (`self.Button Base Mesh`))
  (`StaticMeshComponent.SetStaticMesh` (`self.Button`) (`self.Button Mesh`))
  (bind _returnvalue (`PrimitiveComponent.CreateDynamicMaterialInstance` (`self.Button`) 0 null "None")) ; Make and apply a dynamic material instance for the button
  (bind _output_get (set `self.Button material` _returnvalue)) ; Set the material as a variable for animating
  (`MaterialInstanceDynamic.SetVectorParameterValue` _output_get (`self.Color Parameter Value`) (`self.Button_Color`)) ; Change emissive color of the button
  (if (`self.Trigger is down`)
    (`self.Set Button Position and Color` -1.0 1.0)))