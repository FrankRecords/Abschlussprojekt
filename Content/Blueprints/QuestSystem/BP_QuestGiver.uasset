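; BP_QuestGiver hands a quest to the player through the player character's quest log component.
; Its GiveQuest event queries whether the quest named by its QuestData row is already active and adds it as a new quest only if it is not.
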(event `GiveQuest`
  (if (not (`/Game/Blueprints/QuestSystem/BPC_QuestLogComponent.QueryActiveQuest` (`/Game/Characters/ThirdPerson/Blueprints/BP_ThirdPersonCharacter.BPC_QuestLogComponent` (`/Game/Blueprints/QuestSystem/CommonFunctionLibrary.GetMyPlayerCharacter`)) (`.RowName` (break `DataTableRowHandle` (`self.QuestData`)))))
    (`/Game/Blueprints/QuestSystem/BPC_QuestLogComponent.AddNewQuest` (`/Game/Characters/ThirdPerson/Blueprints/BP_ThirdPersonCharacter.BPC_QuestLogComponent` (`/Game/Blueprints/QuestSystem/CommonFunctionLibrary.GetMyPlayerCharacter`)) (`.RowName` (break `DataTableRowHandle` (`self.QuestData`))))))

(fn `UserConstructionScript`)