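; Base quest Blueprint that tracks a player's progress through one multi-stage quest defined by a row in DT_QuestData.
; It loads the current stage's objectives into a progress map and listens for objective ID events from the player character to increment their counts.
; Finished objectives show a notification widget, and completed stages advance to the next.
; After the last stage it marks the quest completed and, if auto-complete is set, turns it in through BPC_QuestLogComponent.
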(event `self.ReceiveBeginPlay`
  (`self.GetQuestDetails`)
  (add `/Game/Characters/ThirdPerson/Blueprints/BP_ThirdPersonCharacter.OnObjectiveIDCalled` (`/Game/Blueprints/QuestSystem/CommonFunctionLibrary.GetMyPlayerCharacter`) (`|CreateDelegate` :!event `On Objective IDHeard`))
  (bind _return (`self.Are Objectives Complete`))
  (set `self.IsCompleted` _return))

(fn `Are Objectives Complete`
  (returns (Return :type Boolean))
  (locals (LocalBoolComplete :type Boolean :default true))
  (for _array_element (`.Objectives_18_C562142A4667907D9056F2999D3C4C82` (break `/Game/Blueprints/QuestSystem/S_StageDetails` (`self.CurrentStageDetails`)))
    (bind (_objectivename _description _type _objectiveid) (break `/Game/Blueprints/QuestSystem/S_ObjectiveDetails` _array_element))
    (if (not (>= (`BlueprintMapLibrary.Map_Find` (`self.CurrentObjectiveProgress`) _objectiveid) (`.Quantity_14_5DF608084A059B823968F29C3A3265E2` (break `/Game/Blueprints/QuestSystem/S_ObjectiveDetails` (`self.GetObjectiveDataByID` _objectiveid)))))
      (bind _output_get (set `local.LocalBoolComplete` false))
      (return _output_get)))
  (return (`local.LocalBoolComplete`)))

(fn `GetObjectiveDataByID`
  (params (ObjectiveID :type String))
  (returns (`Array Element` :type "/Game/Blueprints/QuestSystem/S_ObjectiveDetails Structure"))
  (for _array_element (`.Objectives_18_C562142A4667907D9056F2999D3C4C82` (break `/Game/Blueprints/QuestSystem/S_StageDetails` (`self.CurrentStageDetails`)))
    (if (`KismetStringLibrary.EqualEqual_StrStr` (`.ObjectiveID_11_CE5EF169494969578A6ABE922730471E` (break `/Game/Blueprints/QuestSystem/S_ObjectiveDetails` _array_element)) ObjectiveID)
      (return _array_element))))

(fn `GetQuestDetails`
  (bind _returnvalue (`|GetDataTableRow` "/Game/Blueprints/QuestSystem/DT_QuestData.DT_QuestData" (`self.QuestID`))
    (:`then`
      (bind _output_get (set `self.QuestDetails` _returnvalue))
      (bind _output_get_2 (set `self.CurrentStageDetails` (`|GetArrayItem` (`.Stages_14_C5D44BDB432CBF8BCE66B7952B221812` (break `/Game/Blueprints/QuestSystem/S_QuestDetails` _output_get)) (`self.CurrentStage`))))
      (`BlueprintMapLibrary.Map_Clear` (`self.CurrentObjectiveProgress`))
      (for _array_element (`.Objectives_18_C562142A4667907D9056F2999D3C4C82` (break `/Game/Blueprints/QuestSystem/S_StageDetails` _output_get_2))
        (`BlueprintMapLibrary.Map_Add` (`self.CurrentObjectiveProgress`) (`.ObjectiveID_11_CE5EF169494969578A6ABE922730471E` (break `/Game/Blueprints/QuestSystem/S_ObjectiveDetails` _array_element)))))))

(fn `IsObjectiveComplete`
  (params (ObjectiveID :type String))
  (bind (_questdetails_questname _questdetails_logdescription _questdetails_trackingdescription _questdetails_ismainquest _questdetails_stages) (break `/Game/Blueprints/QuestSystem/S_QuestDetails` (`self.QuestDetails`)))
  (bind (_objectivename _description _type _objectiveid _quantity) (break `/Game/Blueprints/QuestSystem/S_ObjectiveDetails` (`self.GetObjectiveDataByID` ObjectiveID)))
  (if (>= (`BlueprintMapLibrary.Map_Find` (`self.CurrentObjectiveProgress`) (`local.ObjectiveID`)) _quantity)
    (bind _returnvalue (`|CreateWidget` "/Game/CommonUI/Quest/UI_QuestNotification.UI_QuestNotification_C" null _description))
    (`UserWidget.AddToViewport` _returnvalue 0)
    (bind _return (`self.Are Objectives Complete`))
    (if _return
      (bind _result (`/Engine/EditorBlueprintResources/StandardMacros.IncrementInt` (`self.CurrentStage`))
        (:`  `
          (if (`KismetArrayLibrary.Array_IsValidIndex` _questdetails_stages _result)
            (`self.GetQuestDetails`)
            (else
              (set `self.IsCompleted` true)
              (if (`.AutoComplete_18_64A51E044818CDEC4E6739BEB63B45BC` (break `/Game/Blueprints/QuestSystem/S_QuestDetails` (`self.QuestDetails`)))
                (`/Game/Blueprints/QuestSystem/BPC_QuestLogComponent.TurnInQuest` (`self.GetComponentByClass` (`GameplayStatics.GetPlayerCharacter` 0) "/Game/Blueprints/QuestSystem/BPC_QuestLogComponent.BPC_QuestLogComponent_C") (`self.QuestID`))))))))))

(fn `On Objective IDHeard`
  (params (ObjectiveID :type String))
  (bind (_value _returnvalue) (`BlueprintMapLibrary.Map_Find` (`self.CurrentObjectiveProgress`) ObjectiveID))
  (if _returnvalue
    (if (< _value (`.Quantity_14_5DF608084A059B823968F29C3A3265E2` (break `/Game/Blueprints/QuestSystem/S_ObjectiveDetails` (`self.GetObjectiveDataByID` ObjectiveID))))
      (`BlueprintMapLibrary.Map_Add` (`self.CurrentObjectiveProgress`) ObjectiveID (+ _value 1))
      (`self.IsObjectiveComplete` ObjectiveID)
      (`self.OnObjectiveHeard`)
      (return))
    (else
      (return))))

(fn `UpdateQuestDetails`
  (bind _returnvalue (`|GetDataTableRow` "/Game/Blueprints/QuestSystem/DT_QuestData.DT_QuestData" (`self.QuestID`))
    (:`then`
      (bind _output_get (set `self.QuestDetails` _returnvalue))
      (set `self.CurrentStageDetails` (`|GetArrayItem` (`.Stages_14_C5D44BDB432CBF8BCE66B7952B221812` (break `/Game/Blueprints/QuestSystem/S_QuestDetails` _output_get)) (`self.CurrentStage`))))))

(fn `UserConstructionScript`)