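; Quest-giver component that offers its owning actor's assigned quest to the player and handles showing rewards at turn-in.
; InteractQuest checks the player's quest log, then either auto-accepts a new quest or opens UI_QuestGiver, returning the owner's display name.
; For known quests that are completed but not turned in, it opens UI_QuestRewards.
; Row lookups use DT_QuestData directly, except DisplayQuest, which reads the table from QuestData.
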(fn `DisplayQuest`
  (bind (_datatable _rowname) (break `DataTableRowHandle` (`self.QuestData`)))
  (bind _returnvalue (`|GetDataTableRow` _datatable _rowname)
    (:`then`
      (bind _returnvalue_2 (`|CreateWidget` "/Game/CommonUI/Quest/UI_QuestGiver.UI_QuestGiver_C" null _returnvalue _rowname))
      (`UserWidget.AddToViewport` _returnvalue_2 0))))

(fn `DisplayRewards`
  (bind (_datatable _rowname) (break `DataTableRowHandle` (`self.QuestData`)))
  (bind _returnvalue (`|GetDataTableRow` "/Game/Blueprints/QuestSystem/DT_QuestData.DT_QuestData" _rowname)
    (:`then`
      (bind _returnvalue_2 (`|CreateWidget` "/Game/CommonUI/Quest/UI_QuestRewards.UI_QuestRewards_C" null _returnvalue _rowname))
      (`UserWidget.AddToViewport` _returnvalue_2 0))))

(fn `InteractQuest`
  (returns (ObjectiveID :type String))
  (bind (_datatable _rowname) (break `DataTableRowHandle` (`self.QuestData`)))
  (bind _returnvalue (`Actor.GetComponentByClass` (`GameplayStatics.GetPlayerCharacter` 0) "/Game/Blueprints/QuestSystem/BPC_QuestLogComponent.BPC_QuestLogComponent_C"))
  (bind _returnvalue_2 (`KismetSystemLibrary.GetDisplayName` (`self.GetOwner`)))
  (bind _bpc_questlogcomponent (`/Game/Characters/ThirdPerson/Blueprints/BP_ThirdPersonCharacter.BPC_QuestLogComponent` (`/Game/Blueprints/QuestSystem/CommonFunctionLibrary.GetMyPlayerCharacter`)))
  (if (and (not (`/Game/Blueprints/QuestSystem/BPC_QuestLogComponent.QueryActiveQuest` _bpc_questlogcomponent _rowname)) (not (`/Game/Blueprints/QuestSystem/BPC_QuestLogComponent.QueryCompletedQuests` _bpc_questlogcomponent _rowname)))
    (bind _returnvalue_3 (`|GetDataTableRow` "/Game/Blueprints/QuestSystem/DT_QuestData.DT_QuestData" (`.RowName` (break `DataTableRowHandle` (`self.QuestData`))))
      (:`then`
        (if (`.AutoAccept_16_E78F0A3547F65F939A3B35AF24A86C7E` (break `/Game/Blueprints/QuestSystem/S_QuestDetails` _returnvalue_3))
          (`/Engine/EditorBlueprintResources/StandardMacros.IsValid` _returnvalue
            (:`Is Valid`
              (`/Game/Blueprints/QuestSystem/BPC_QuestLogComponent.AddNewQuest` _returnvalue (`.RowName` (break `DataTableRowHandle` (`self.QuestData`))))
              (return (`KismetSystemLibrary.GetDisplayName` (`self.GetOwner`)))))
          (else
            (`self.DisplayQuest`)
            (return _returnvalue_2)))))
    (else
      (bind _array_element (`/Game/Blueprints/QuestSystem/BPC_QuestLogComponent.GetQuestActor` (`/Game/Characters/ThirdPerson/Blueprints/BP_ThirdPersonCharacter.BPC_QuestLogComponent` (`/Game/Blueprints/QuestSystem/CommonFunctionLibrary.GetMyPlayerCharacter`)) (`.RowName` (break `DataTableRowHandle` (`self.QuestData`)))))
      (if (and (`/Game/Blueprints/QuestSystem/BP_QuestBase.IsCompleted` _array_element) (not (`/Game/Blueprints/QuestSystem/BP_QuestBase.IsTurnedIn` _array_element)))
        (`self.DisplayRewards`)
        (return _returnvalue_2)))))