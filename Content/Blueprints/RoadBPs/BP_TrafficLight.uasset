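; Traffic light actor that cycles on its own between green and red, with a short yellow phase before every change.
; BeginPlay runs an endless delay loop in which a FlipFlop alternates the state after yellow, going to green first.
; Each switch function toggles visibility of paired on/off components per lamp and updates IsTrafficLightGreen, which is true only during green.
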(event `self.ReceiveBeginPlay`
  (`KismetSystemLibrary.Delay` 10.0 :!label _label)
  (`self.SwitchToYellow`)
  (`KismetSystemLibrary.Delay` 2.0)
  (`/Engine/EditorBlueprintResources/StandardMacros.FlipFlop`
    (:`A`
      (`self.SwitchToGreen`)
      (goto _label))
    (:`B`
      (`self.SwitchToRed`)
      (goto _label))))

(fn `SwitchToGreen`
  (set `self.bIsTrafficLightGreen` true)
  (`|ExecutionSequence`
    (:`then_0`
      (`SceneComponent.SetHiddenInGame` (`self.GreenLightOn`) false false)
      (`SceneComponent.SetHiddenInGame` (`self.YellowLightOff`) false false)
      (`SceneComponent.SetHiddenInGame` (`self.RedLightOff`) false false))
    (:`then_1`
      (`SceneComponent.SetHiddenInGame` (`self.GreenLightOff`) true false)
      (`SceneComponent.SetHiddenInGame` (`self.YellowLightOn`) true false)
      (`SceneComponent.SetHiddenInGame` (`self.RedLightOn`) true false))))

(fn `SwitchToRed`
  (set `self.bIsTrafficLightGreen` false)
  (`|ExecutionSequence`
    (:`then_0`
      (`SceneComponent.SetHiddenInGame` (`self.RedLightOn`) false false)
      (`SceneComponent.SetHiddenInGame` (`self.YellowLightOff`) false false)
      (`SceneComponent.SetHiddenInGame` (`self.GreenLightOff`) false false))
    (:`then_1`
      (`SceneComponent.SetHiddenInGame` (`self.GreenLightOn`) true false)
      (`SceneComponent.SetHiddenInGame` (`self.RedLightOff`) true false)
      (`SceneComponent.SetHiddenInGame` (`self.YellowLightOn`) true false))))

(fn `SwitchToYellow`
  (set `self.bIsTrafficLightGreen` false)
  (`|ExecutionSequence`
    (:`then_0`
      (`SceneComponent.SetHiddenInGame` (`self.YellowLightOn`) false false)
      (`SceneComponent.SetHiddenInGame` (`self.GreenLightOff`) false false)
      (`SceneComponent.SetHiddenInGame` (`self.RedLightOff`) false false))
    (:`then_1`
      (`SceneComponent.SetHiddenInGame` (`self.RedLightOn`) true false)
      (`SceneComponent.SetHiddenInGame` (`self.GreenLightOn`) true false)
      (`SceneComponent.SetHiddenInGame` (`self.YellowLightOff`) true false))))

(fn `UserConstructionScript`)