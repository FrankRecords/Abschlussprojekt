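; Spline road actor for AI traffic, built to spawn random data-table cars along its length by player distance.
; Polling is meant to alternate spawning and despawning, with cars tracked in an array and handed a road reference.
; As shown, BeginPlay and most event bodies are unwired, so that loop never starts.
; The construction script optionally lays spline-mesh arrows, coloring the last few red to mark the end.
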(event `self.ReceiveBeginPlay`
  ;[0 0 0] BeginPlay
)

(event `DespawnCar`
  ;[0 0.1211 1] SpawnAndDespawn Cars
)

(event `RemoveCarOldSpline`
  (params (Item :type "/Game/Blueprints/CarBPs/BP_AI-Car Object Reference (by ref)"))
  ;[0 0.1211 1] SpawnAndDespawn Cars
)

(event `AddCarCurrentSpline`
  (params (NewItem :type "/Game/Blueprints/CarBPs/BP_AI-Car Object Reference (by ref)"))
  ;[0 0.1211 1] SpawnAndDespawn Cars
)

(event `SpawnCars`
  (params (Amount :type Integer))
  ;[0 0.1211 1] SpawnAndDespawn Cars
)

(event `CheckForSpawn`
  (bind _returnvalue (`self.GetDistanceToPlayer`))
  ;[0 0.1211 1] SpawnAndDespawn Cars
  (if (< _returnvalue (`self.SpawnDistance`)) :!label _label
    (`self.SpawnCars` (`self.AmountSpawn`))
    (`KismetSystemLibrary.Delay` 1.0)
    (`self.CheckForDespawn`)
    (else
      (`KismetSystemLibrary.Delay` (/ _returnvalue 3000.0))
      (goto _label))))

(event `CheckForDespawn`
  ;[0 0.1211 1] SpawnAndDespawn Cars
)

(fn `DivideSplineLenght`
  (params (Amount :type Integer))
  (set `self.SplineLenghtALL` (/ (`SplineComponent.GetSplineLength` (`self.Spline`)) Amount))
  (for _index (range (+ Amount 1))
    (`KismetArrayLibrary.Array_Add` (`self.PointSpawmToLenght`) (`KismetMathLibrary.FClamp` (* _index (`self.SplineLenghtALL`)) 1000.0 (- (`SplineComponent.GetSplineLength` (`self.Spline`)) 1000.0)))))

(fn `GetAllCarsDataBase`
  (bind _outrownames (`DataTableFunctionLibrary.GetDataTableRowNames` "/Game/Blueprints/CarBPs/D_AI-Cars.D_AI-Cars"))
  (for _array_element _outrownames
    (bind _returnvalue (`|GetDataTableRow` "/Game/Blueprints/CarBPs/D_AI-Cars.D_AI-Cars" _array_element)
      (:`then`
        (bind (_car _randomcolor) (break `/Game/Blueprints/CarBPs/S_AI-Cars` _returnvalue))
        (if (`KismetSystemLibrary.IsValidClass` _car)
          (`KismetArrayLibrary.Array_Add` (`self.AllCars`) _car)
          (`KismetArrayLibrary.Array_Add` (`self.Random Color`) _randomcolor))))))

(fn `GetDistanceToPlayer`
  (returns (ReturnValue :type "Float (single-precision)"))
  (return (`self.GetDistanceTo` (`GameplayStatics.GetPlayerCharacter` 0))))

(fn `Set ColorLastArrow`
  (params (Index :type Integer))
  (returns (ReturnValue :type Boolean))
  (return (or (== Index (`self.NumberInstances`)) (== Index (- (`self.NumberInstances`) 1)) (== Index (- (`self.NumberInstances`) 2)) (== Index (- (`self.NumberInstances`) 3)))))

(fn `SpawnCarSelect`
  (params (LocationSpline :type "Float (single-precision)"))
  (bind _allcars (`self.AllCars`))
  (bind _spline (`self.Spline`))
  (bind _returnvalue (`KismetMathLibrary.RandomIntegerInRange` 0 (- (`KismetArrayLibrary.Array_Length` _allcars) 1)))
  (bind _returnvalue_2 (`|SpawnActorFromClass` (`|GetArrayItem` _allcars _returnvalue) (`KismetMathLibrary.MakeTransform` (`SplineComponent.GetLocationAtDistanceAlongSpline` _spline LocationSpline "World") (`SplineComponent.GetRotationAtDistanceAlongSpline` _spline LocationSpline "World")) "Undefined" "SelectDefaultAtRuntime" null null (`|GetArrayItem` (`self.Random Color`) _returnvalue) null))
  (`/Engine/EditorBlueprintResources/StandardMacros.IsValid` _returnvalue_2
    (:`Is Valid`
      (message `/Game/Blueprints/RoadBPs/BPI_CarTrafficAI_System.SetRoad` _returnvalue_2 self)
      (`KismetArrayLibrary.Array_Add` (`self.SpawnedAI`) _returnvalue_2))))

(fn `UserConstructionScript`
  (bind _spline (`self.Spline`))
  (bind _meshsize (`self.MeshSize`))
  (bind _spline_2 (`self.Spline`))
  (bind _returnvalue (`KismetMathLibrary.FTrunc` (/ (`SplineComponent.GetSplineLength` (`self.Spline`)) (`self.MeshSize`))))
  (if (`self.ShowArrows?`)
    (set `self.NumberInstances` _returnvalue)
    (for _index (range (+ _returnvalue 1))
      (bind _returnvalue_2 (* _index _meshsize))
      (bind _returnvalue_3 (+ _returnvalue_2 _meshsize))
      (if (not (> _returnvalue_3 (`SplineComponent.GetSplineLength` (`self.Spline`))))
        (bind _returnvalue_4 (`AddComponent|NODE_AddSplineMeshComponent-4`))
        (`SplineMeshComponent.SetStartAndEnd` _returnvalue_4 (`SplineComponent.GetLocationAtDistanceAlongSpline` _spline _returnvalue_2 "Local") (`KismetMathLibrary.ClampVectorSize` (`SplineComponent.GetTangentAtDistanceAlongSpline` _spline _returnvalue_2 "Local") 0.0 (`self.MeshSize`)) (`SplineComponent.GetLocationAtDistanceAlongSpline` _spline_2 _returnvalue_3 "Local") (`KismetMathLibrary.ClampVectorSize` (`SplineComponent.GetTangentAtDistanceAlongSpline` _spline_2 _returnvalue_3 "Local") 0.0 (`self.MeshSize`)) true)
        (bind _returnvalue_5 (`self.Set ColorLastArrow` _index))
        (if _returnvalue_5
          (bind _returnvalue_6 (`PrimitiveComponent.CreateDynamicMaterialInstance` _returnvalue_4 0 "/Game/TrafficAISystem/Blueprints/Material/M_Arrow.M_Arrow" "None"))
          (`MaterialInstanceDynamic.SetVectorParameterValue` _returnvalue_6 "Color" (struct :`R` 0.630208 :`B` 0.015696 :`A` 1.0)))))))