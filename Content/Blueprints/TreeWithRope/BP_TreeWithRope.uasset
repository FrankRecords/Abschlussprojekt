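; Tree rope puzzle where the player hoists and drops a stone to complete the Squirrel quest.
; An overlapping rope-with-stone item is consumed, revealing the rig during a brief camera cutscene and reporting an objective.
; Interacting attaches the rope end to the player; holding pull raises the stone by timeline, and letting go reverses it.
; A full pull turns the Geometry Collection into a Chaos physics object, releases the rope and shakes the camera.
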(event `self.ReceiveBeginPlay`
  (set `self.StartLocation` (`SceneComponent.RelativeLocation` (`self.GeometryCollection`)))
  (bind _asbp_third_person_character (cast `/Game/Characters/ThirdPerson/Blueprints/BP_ThirdPersonCharacter` (`GameplayStatics.GetPlayerCharacter` 0)))
  (set `self.PlayerRef` _asbp_third_person_character))

(event `self.ActivateRock.OnComponentBeginOverlap`
  (params (OverlappedComponent :type "PrimitiveComponent Object Reference") (OtherActor :type "Actor Object Reference") (OtherComp :type "PrimitiveComponent Object Reference") (OtherBodyIndex :type Integer) (bFromSweep :type Boolean) (SweepResult :type "HitResult Structure (by ref)"))
  (bind _asbp_equip_item_rope_with_stone (cast `/Game/CommonUI/03_Inventory/ItemClasses/BP_EquipItem_RopeWithStone` OtherActor))
  (`PlayerController.SetViewTargetWithBlend` (`GameplayStatics.GetPlayerController` 0) self 0.5 "VTBlend_Cubic" 0.0 false)
  (`|ExecutionSequence`
    (:`then_0`
      (`CharacterMovementComponent.DisableMovement` (`Character.CharacterMovement` (`GameplayStatics.GetPlayerCharacter` 0)))
      (bind (_direction _movecameratrack) (`Timeline|Movecamera` :!via `PlayFromStart`)
        (:`Update`
          (`SceneComponent.K2_SetRelativeLocation` (`self.Camera`) (`KismetMathLibrary.VLerp` (-950.0 70.0 250.0) (-950.0 70.0 650.0) _movecameratrack) false false))))
    (:`then_1`
      (`KismetSystemLibrary.Delay` 0.2)
      (`self.K2_DestroyActor` _asbp_equip_item_rope_with_stone)
      (`SceneComponent.SetHiddenInGame` (`self.GeometryCollection`) false false)
      (`SceneComponent.SetHiddenInGame` (`self.RopeStone`) false false)
      (`SceneComponent.SetHiddenInGame` (`self.RopePull`) false false)
      (`PrimitiveComponent.SetEnableGravity` (`self.RopeEndPull`) true)
      (`PrimitiveComponent.SetCollisionEnabled` (`self.BLOCKBOTTOM`) "NoCollision")
      (`KismetSystemLibrary.Delay` 3.0)
      (`PlayerController.SetViewTargetWithBlend` (`GameplayStatics.GetPlayerController` 0) (`GameplayStatics.GetPlayerCharacter` 0) 1.0 "VTBlend_Cubic" 0.0 false)
      (`CharacterMovementComponent.SetMovementMode` (`Character.CharacterMovement` (`GameplayStatics.GetPlayerCharacter` 0)) "MOVE_Walking" 0)
      (`/Game/Characters/ThirdPerson/Blueprints/BP_ThirdPersonCharacter.OnObjectiveIDCalled` (`/Game/Blueprints/QuestSystem/CommonFunctionLibrary.GetMyPlayerCharacter`) (`self.ObjectiveID`)))))

(event `EnhancedInput|/Game/CommonUI/Foundation/Input/EnhancedInput/Actions/IA_UI_PullRope`
  (params (ActionValue :type Boolean) (ElapsedSeconds :type "Float (double-precision)") (TriggeredSeconds :type "Float (double-precision)") (InputAction :type "InputAction Object Reference" :default "/Game/CommonUI/Foundation/Input/EnhancedInput/Actions/IA_UI_PullRope.IA_UI_PullRope"))
  (:`Triggered`
    (set `/Game/Characters/ThirdPerson/Blueprints/BP_ThirdPersonCharacter.isPullingRope` true (`self.PlayerRef`))
    (if (not (`self.DropCompleted?`))
      (bind (_direction _pullupstone) (`Timeline|PullUpStone` :!label _label)
        (:`Update`
          (`SceneComponent.K2_SetRelativeLocation` (`self.GeometryCollection`) (`KismetMathLibrary.VLerp` (`self.StartLocation`) (`self.EndLocation`) _pullupstone) false false))
        (:`Finished`
          (if (> _pullupstone 0.9)
            (set `GeometryCollectionComponent.ObjectType` "Chaos_Object_Dynamic" (`self.GeometryCollection`))
            (`PrimitiveComponent.SetSimulatePhysics` (`self.GeometryCollection`) true)
            (set `self.DropCompleted?` true)
            (`self.DropRope`)
            (`/Game/Characters/ThirdPerson/Blueprints/BP_ThirdPersonCharacter.OnObjectiveIDCalled` (`/Game/Blueprints/QuestSystem/CommonFunctionLibrary.GetMyPlayerCharacter`) "nutdropping")
            (`KismetSystemLibrary.Delay` 0.8)
            (`PlayerController.ClientStartCameraShake` :`self` (`GameplayStatics.GetPlayerController` 0) :`Shake` "/Game/Characters/ThirdPerson/Blueprints/BP_CameraShake.BP_CameraShake_C")
            (`/Game/Blueprints/QuestSystem/BPC_QuestLogComponent.TurnInQuest` (`self.GetComponentByClass` (`GameplayStatics.GetPlayerCharacter` 0) "/Game/Blueprints/QuestSystem/BPC_QuestLogComponent.BPC_QuestLogComponent_C") "Squirrel"))))))
  (:`Canceled`
    (set `/Game/Characters/ThirdPerson/Blueprints/BP_ThirdPersonCharacter.isPullingRope` false (`self.PlayerRef`) :!label _label_2)
    (goto _label :!via `Reverse`))
  (:`Completed`
    (goto _label_2)))

(event `EnhancedInput|/Game/CommonUI/Foundation/Input/EnhancedInput/Actions/IA_UI_Release`
  (params (ActionValue :type Boolean) (ElapsedSeconds :type "Float (double-precision)") (TriggeredSeconds :type "Float (double-precision)") (InputAction :type "InputAction Object Reference" :default "/Game/CommonUI/Foundation/Input/EnhancedInput/Actions/IA_UI_Release.IA_UI_Release"))
  (bind _ropeendpull (`self.RopeEndPull`))
  (:`Triggered`
    (`|ExecutionSequence`
      (:`then_0`
        (set `/Game/Characters/ThirdPerson/Blueprints/BP_ThirdPersonCharacter.isPullingRope` false (`self.PlayerRef`))
        (goto _label :!via `Reverse`))
      (:`then_1`
        (`SceneComponent.K2_DetachFromComponent` _ropeendpull "KeepWorld" "KeepWorld" "KeepWorld" true :!label _label_3)
        (`PrimitiveComponent.SetSimulatePhysics` _ropeendpull true)
        (`self.DisableInput` (`GameplayStatics.GetPlayerController` 0))
        (`PrimitiveComponent.SetCollisionEnabled` (`self.Sphere`) "QueryOnly")
        (set `/Game/Characters/ThirdPerson/Blueprints/BP_ThirdPersonCharacter.isPullingRope` false (`self.PlayerRef`))
        (set `self.HasRope` false)
        (`/Game/CommonUI/11_Tutorial/UI_KeysHintPull.RemoveWidget` (`self.KeysHintWidget`))))))

(event `DropRope`
  (goto _label_3))

(event `/Game/Blueprints/Interfaces/BPI_Interact.Interaction`
  (params (CharacterRef :type "/Game/Characters/ThirdPerson/Blueprints/BP_ThirdPersonCharacter Object Reference"))
  (bind _ropeendpull (`self.RopeEndPull`))
  (if (not (`self.DropCompleted?`))
    (`PrimitiveComponent.SetSimulatePhysics` _ropeendpull false)
    (`SceneComponent.K2_AttachToComponent` _ropeendpull (`Character.Mesh` CharacterRef) "Items" "SnapToTarget" "KeepWorld" "KeepWorld" true)
    (`self.EnableInput` (`GameplayStatics.GetPlayerController` 0))
    (`PrimitiveComponent.SetCollisionEnabled` (`self.Sphere`) "NoCollision")
    (set `self.HasRope` true)
    (`SceneComponent.SetVisibility` (`self.InteractWidget`) false false)
    (bind _returnvalue (`|CreateWidget` "/Game/CommonUI/11_Tutorial/UI_KeysHintPull.UI_KeysHintPull_C"))
    (bind _output_get (set `self.KeysHintWidget` _returnvalue))
    (`UserWidget.AddToViewport` _output_get 0)))

(event `self.IconTrigger.OnComponentBeginOverlap`
  (params (OverlappedComponent :type "PrimitiveComponent Object Reference") (OtherActor :type "Actor Object Reference") (OtherComp :type "PrimitiveComponent Object Reference") (OtherBodyIndex :type Integer) (bFromSweep :type Boolean) (SweepResult :type "HitResult Structure (by ref)"))
  (if (`self.ActorHasTag` OtherActor "Player")
    (if (not (`self.HasRope`))
      (`SceneComponent.SetVisibility` (`self.InteractWidget`) true false))))

(event `self.IconTrigger.OnComponentEndOverlap`
  (params (OverlappedComponent :type "PrimitiveComponent Object Reference") (OtherActor :type "Actor Object Reference") (OtherComp :type "PrimitiveComponent Object Reference") (OtherBodyIndex :type Integer))
  (if (`self.ActorHasTag` OtherActor "Player")
    (`SceneComponent.SetVisibility` (`self.InteractWidget`) false false)))

(fn `UserConstructionScript`)