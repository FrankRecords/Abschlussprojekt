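; Dissolve box actor that publishes its box's location, scale and axis vectors to the MPC_Box2_Data material parameter collection, presumably driving object-based dissolve materials.
; The construction script and BeginPlay write these values once.
; MoveBoxInWorld or TransitionWorld starts a looping timer that refreshes them while a timeline lerps the actor to NewLocation.
; On finish it clears the timer and swaps start and target, so each call toggles position.
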(event `ActivateUpdateVector`
  (bind _returnvalue (`KismetSystemLibrary.K2_SetTimerDelegate` (delegate `UpdateVectorParameters`) 0.01 true true))
  (set `self.ActiveTimer` _returnvalue))

(event `UpdateVectorParameters`
  (bind _box (`self.Box`))
  (bind _box_2 (`self.Box`))
  (`KismetMaterialLibrary.SetVectorParameterValue` "/Game/Blueprints/DissolveByObject/MPC_Box2_Data.MPC_Box2_Data" "Location" (`KismetMathLibrary.Conv_VectorToLinearColor` (`SceneComponent.K2_GetComponentLocation` _box)) :!label _label)
  (`KismetMaterialLibrary.SetVectorParameterValue` "/Game/Blueprints/DissolveByObject/MPC_Box2_Data.MPC_Box2_Data" "Bounds" (`KismetMathLibrary.Conv_VectorToLinearColor` (`SceneComponent.K2_GetComponentScale` _box)))
  (`KismetMaterialLibrary.SetVectorParameterValue` "/Game/Blueprints/DissolveByObject/MPC_Box2_Data.MPC_Box2_Data" "X" (`KismetMathLibrary.Conv_VectorToLinearColor` (`SceneComponent.GetForwardVector` _box_2)))
  (`KismetMaterialLibrary.SetVectorParameterValue` "/Game/Blueprints/DissolveByObject/MPC_Box2_Data.MPC_Box2_Data" "Y" (`KismetMathLibrary.Conv_VectorToLinearColor` (`SceneComponent.GetRightVector` _box_2)))
  (`KismetMaterialLibrary.SetVectorParameterValue` "/Game/Blueprints/DissolveByObject/MPC_Box2_Data.MPC_Box2_Data" "Z" (`KismetMathLibrary.Conv_VectorToLinearColor` (`SceneComponent.GetUpVector` _box_2))))

(event `self.ReceiveBeginPlay`
  (`|ExecutionSequence`
    (:`then_0`
      (goto _label))
    (:`then_1`
      (set `self.StartLocation` (`self.K2_GetActorLocation`)))))

(event `ClearTimer`
  (`KismetSystemLibrary.K2_ClearAndInvalidateTimerHandle` (`self.ActiveTimer`)))

(event `MoveBoxInWorld`
  (`self.ActivateUpdateVector` :!label _label_2)
  (bind (_direction _scale) (`Timeline|Timeline` :!via `PlayFromStart`)
    (:`Update`
      (`self.K2_SetActorLocation` (`KismetMathLibrary.VLerp` (`self.StartLocation`) (`self.NewLocation`) _scale)))
    (:`Finished`
      (`self.ClearTimer`)
      (set `self.StoreLocation` (`self.StartLocation`))
      (set `self.StartLocation` (`self.NewLocation`))
      (set `self.NewLocation` (`self.StoreLocation`)))))

(event `/Game/Blueprints/Interfaces/BPI_TransitionWorld.TransitionWorld`
  (goto _label_2))

(fn `UserConstructionScript`
  (bind _box (`self.Box`))
  (bind _box_2 (`self.Box`))
  (`KismetMaterialLibrary.SetVectorParameterValue` "/Game/Blueprints/DissolveByObject/MPC_Box2_Data.MPC_Box2_Data" "Location" (`KismetMathLibrary.Conv_VectorToLinearColor` (`SceneComponent.K2_GetComponentLocation` _box)))
  (`KismetMaterialLibrary.SetVectorParameterValue` "/Game/Blueprints/DissolveByObject/MPC_Box2_Data.MPC_Box2_Data" "Bounds" (`KismetMathLibrary.Conv_VectorToLinearColor` (`SceneComponent.K2_GetComponentScale` _box)))
  (`KismetMaterialLibrary.SetVectorParameterValue` "/Game/Blueprints/DissolveByObject/MPC_Box2_Data.MPC_Box2_Data" "X" (`KismetMathLibrary.Conv_VectorToLinearColor` (`SceneComponent.GetForwardVector` _box_2)))
  (`KismetMaterialLibrary.SetVectorParameterValue` "/Game/Blueprints/DissolveByObject/MPC_Box2_Data.MPC_Box2_Data" "Y" (`KismetMathLibrary.Conv_VectorToLinearColor` (`SceneComponent.GetRightVector` _box_2)))
  (`KismetMaterialLibrary.SetVectorParameterValue` "/Game/Blueprints/DissolveByObject/MPC_Box2_Data.MPC_Box2_Data" "Z" (`KismetMathLibrary.Conv_VectorToLinearColor` (`SceneComponent.GetUpVector` _box_2))))