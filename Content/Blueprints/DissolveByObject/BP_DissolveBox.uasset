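; Dissolve box that drives a one-time, saved transition from the real world to the dream world.
; It writes location, scale and axes to MPC_Box_Data, presumably for dissolve materials.
; TransitionWorld starts a looping timer that lerps the location along a Timeline with emissive on, later disabling RealWorld foliage collision.
; BeginPlay requests saved state, then restores the box parameters and disables collision on the inactive world's tagged foliage.
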(event `ActivateUpdateVector`
  (bind _returnvalue (`KismetSystemLibrary.K2_SetTimerDelegate` (delegate `UpdateVectorParameters`) 0.001 true true))
  (set `self.ActiveTimer` _returnvalue)
  (bind (_direction _alpha) (`Timeline|Timeline` :!via `PlayFromStart`)))

(event `UpdateVectorParameters`
  (bind _box (`self.Box`))
  (`KismetMaterialLibrary.SetVectorParameterValue` "/Game/Blueprints/DissolveByObject/MPC_Box_Data.MPC_Box_Data" "Location" (`KismetMathLibrary.Conv_VectorToLinearColor` (`KismetMathLibrary.VLerp` (`self.StartPosition`) (`self.EndPosition`) (stale `ActivateUpdateVector` _alpha))))
  (`KismetMaterialLibrary.SetVectorParameterValue` "/Game/Blueprints/DissolveByObject/MPC_Box_Data.MPC_Box_Data" "Bounds" (`KismetMathLibrary.Conv_VectorToLinearColor` (`SceneComponent.K2_GetComponentScale` (`self.Box`))) :!label _label)
  (`KismetMaterialLibrary.SetVectorParameterValue` "/Game/Blueprints/DissolveByObject/MPC_Box_Data.MPC_Box_Data" "X" (`KismetMathLibrary.Conv_VectorToLinearColor` (`SceneComponent.GetForwardVector` _box)))
  (`KismetMaterialLibrary.SetVectorParameterValue` "/Game/Blueprints/DissolveByObject/MPC_Box_Data.MPC_Box_Data" "Y" (`KismetMathLibrary.Conv_VectorToLinearColor` (`SceneComponent.GetRightVector` _box)))
  (`KismetMaterialLibrary.SetVectorParameterValue` "/Game/Blueprints/DissolveByObject/MPC_Box_Data.MPC_Box_Data" "Z" (`KismetMathLibrary.Conv_VectorToLinearColor` (`SceneComponent.GetUpVector` _box))))

(event `self.ReceiveBeginPlay`
  (message `/Game/Blueprints/SaveGame/BPI_Persistence.RequestLoad` (`GameplayStatics.GetGameInstance`) self)
  (`KismetSystemLibrary.Delay` 0.2)
  (`|ExecutionSequence`
    (:`then_0`
      (if (`self.TransitionTriggered?`)
        (`KismetMaterialLibrary.SetVectorParameterValue` "/Game/Blueprints/DissolveByObject/MPC_Box_Data.MPC_Box_Data" "Location" (`KismetMathLibrary.Conv_VectorToLinearColor` (`self.EndPosition`)))
        (`KismetMaterialLibrary.SetScalarParameterValue` "/Game/Blueprints/DissolveByObject/MPC_Box_Data.MPC_Box_Data" "EmissiveBool")
        (goto _label)
        (else
          (`KismetMaterialLibrary.SetVectorParameterValue` "/Game/Blueprints/DissolveByObject/MPC_Box_Data.MPC_Box_Data" "Location" (`KismetMathLibrary.Conv_VectorToLinearColor` (`self.StartPosition`)))
          (goto _label))))
    (:`then_1`
      (if (`self.TransitionTriggered?`)
        (`KismetSystemLibrary.Delay` 0.1)
        (bind _outactors (`GameplayStatics.GetAllActorsOfClass` "/Script/Foliage.InstancedFoliageActor"))
        (for _array_element _outactors
          (if (`self.ActorHasTag` _array_element "TransitionFoliage")
            (for _array_element_2 (`self.GetComponentsByTag` _array_element "/Script/Foliage.FoliageInstancedStaticMeshComponent" "RealWorld")
              (`PrimitiveComponent.SetCollisionEnabled` _array_element_2 "NoCollision"))))
        (else
          (`KismetSystemLibrary.Delay` 0.1)
          (bind _outactors_2 (`GameplayStatics.GetAllActorsOfClass` "/Script/Foliage.InstancedFoliageActor"))
          (for _array_element_3 _outactors_2
            (if (`self.ActorHasTag` _array_element_3 "TransitionFoliage")
              (for _array_element_4 (`self.GetComponentsByTag` _array_element_3 "/Script/Foliage.FoliageInstancedStaticMeshComponent" "DreamWorld")
                (`PrimitiveComponent.SetCollisionEnabled` _array_element_4 "NoCollision")))))))))

(event `ClearTimer`
  (`KismetSystemLibrary.K2_ClearAndInvalidateTimerHandle` (`self.ActiveTimer`)))

(event `/Game/Blueprints/Interfaces/BPI_TransitionWorld.TransitionWorld`
  (if (not (`self.TransitionTriggered?`))
    (`self.ActivateUpdateVector`)
    (`KismetMaterialLibrary.SetScalarParameterValue` "/Game/Blueprints/DissolveByObject/MPC_Box_Data.MPC_Box_Data" "EmissiveBool" 1.0)
    (set `self.TransitionTriggered?` true)
    (`|ExecutionSequence`
      (:`then_0`
        (`KismetSystemLibrary.Delay` 15.0)
        (`self.ClearTimer`)
        (`KismetMaterialLibrary.SetScalarParameterValue` "/Game/Blueprints/DissolveByObject/MPC_Box_Data.MPC_Box_Data" "EmissiveBool"))
      (:`then_1`
        (`KismetSystemLibrary.Delay` 5.0)
        (bind _outactors (`GameplayStatics.GetAllActorsOfClass` "/Script/Foliage.InstancedFoliageActor"))
        (for _array_element _outactors
          (if (`self.ActorHasTag` _array_element "TransitionFoliage")
            (for _array_element_2 (`self.GetComponentsByTag` _array_element "/Script/Foliage.FoliageInstancedStaticMeshComponent" "RealWorld")
              (`PrimitiveComponent.SetCollisionEnabled` _array_element_2 "NoCollision"))))))))

(event `/Game/Blueprints/SaveGame/BPI_Saveable.LoadData`
  (params (SaveGameRef :type "/Game/Blueprints/SaveGame/BP_SaveGame Object Reference"))
  (set `self.TransitionTriggered?` (`/Game/Blueprints/SaveGame/BP_SaveGame.TransitionTriggered?` SaveGameRef)))

(event `/Game/Blueprints/SaveGame/BPI_Saveable.SaveData`
  (params (SaveGameRef :type "/Game/Blueprints/SaveGame/BP_SaveGame Object Reference"))
  (set `/Game/Blueprints/SaveGame/BP_SaveGame.TransitionTriggered?` (`self.TransitionTriggered?`) SaveGameRef))

(fn `UserConstructionScript`
  (bind _box (`self.Box`))
  (bind _box_2 (`self.Box`))
  (`KismetMaterialLibrary.SetVectorParameterValue` "/Game/Blueprints/DissolveByObject/MPC_Box_Data.MPC_Box_Data" "Location" (`KismetMathLibrary.Conv_VectorToLinearColor` (`SceneComponent.K2_GetComponentLocation` _box)))
  (`KismetMaterialLibrary.SetVectorParameterValue` "/Game/Blueprints/DissolveByObject/MPC_Box_Data.MPC_Box_Data" "Bounds" (`KismetMathLibrary.Conv_VectorToLinearColor` (`SceneComponent.K2_GetComponentScale` _box)))
  (`KismetMaterialLibrary.SetVectorParameterValue` "/Game/Blueprints/DissolveByObject/MPC_Box_Data.MPC_Box_Data" "X" (`KismetMathLibrary.Conv_VectorToLinearColor` (`SceneComponent.GetForwardVector` _box_2)))
  (`KismetMaterialLibrary.SetVectorParameterValue` "/Game/Blueprints/DissolveByObject/MPC_Box_Data.MPC_Box_Data" "Y" (`KismetMathLibrary.Conv_VectorToLinearColor` (`SceneComponent.GetRightVector` _box_2)))
  (`KismetMaterialLibrary.SetVectorParameterValue` "/Game/Blueprints/DissolveByObject/MPC_Box_Data.MPC_Box_Data" "Z" (`KismetMathLibrary.Conv_VectorToLinearColor` (`SceneComponent.GetUpVector` _box_2))))