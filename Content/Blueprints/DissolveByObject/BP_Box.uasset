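; Box actor that publishes its transform to the MPC_Box_Data material parameter collection, apparently to drive a dissolve-by-object effect in materials.
; It writes world location, scale as bounds, and forward, right and up axes, describing an oriented box.
; The construction script and BeginPlay each push the values once.
; ActivateUpdateVector starts a fast looping timer that keeps them refreshed while the box moves, and ClearTimer stops it.
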(event `ActivateUpdateVector`
  (bind _returnvalue (`KismetSystemLibrary.K2_SetTimerDelegate` (delegate `UpdateVectorParameters`) 0.05 true true))
  (set `self.ActiveTimer` _returnvalue))

(event `UpdateVectorParameters`
  (bind _box (`self.Box`))
  (bind _box_2 (`self.Box`))
  (`KismetMaterialLibrary.SetVectorParameterValue` "/Game/Blueprints/DissolveByObject/MPC_Box_Data.MPC_Box_Data" "Location" (`KismetMathLibrary.Conv_VectorToLinearColor` (`SceneComponent.K2_GetComponentLocation` _box)) :!label _label)
  (`KismetMaterialLibrary.SetVectorParameterValue` "/Game/Blueprints/DissolveByObject/MPC_Box_Data.MPC_Box_Data" "Bounds" (`KismetMathLibrary.Conv_VectorToLinearColor` (`SceneComponent.K2_GetComponentScale` _box)))
  (`KismetMaterialLibrary.SetVectorParameterValue` "/Game/Blueprints/DissolveByObject/MPC_Box_Data.MPC_Box_Data" "X" (`KismetMathLibrary.Conv_VectorToLinearColor` (`SceneComponent.GetForwardVector` _box_2)))
  (`KismetMaterialLibrary.SetVectorParameterValue` "/Game/Blueprints/DissolveByObject/MPC_Box_Data.MPC_Box_Data" "Y" (`KismetMathLibrary.Conv_VectorToLinearColor` (`SceneComponent.GetRightVector` _box_2)))
  (`KismetMaterialLibrary.SetVectorParameterValue` "/Game/Blueprints/DissolveByObject/MPC_Box_Data.MPC_Box_Data" "Z" (`KismetMathLibrary.Conv_VectorToLinearColor` (`SceneComponent.GetUpVector` _box_2))))

(event `self.ReceiveBeginPlay`
  (goto _label))

(event `ClearTimer`
  (`KismetSystemLibrary.K2_ClearAndInvalidateTimerHandle` (`self.ActiveTimer`)))

(fn `UserConstructionScript`
  (bind _box (`self.Box`))
  (bind _box_2 (`self.Box`))
  (`KismetMaterialLibrary.SetVectorParameterValue` "/Game/Blueprints/DissolveByObject/MPC_Box_Data.MPC_Box_Data" "Location" (`KismetMathLibrary.Conv_VectorToLinearColor` (`SceneComponent.K2_GetComponentLocation` _box)))
  (`KismetMaterialLibrary.SetVectorParameterValue` "/Game/Blueprints/DissolveByObject/MPC_Box_Data.MPC_Box_Data" "Bounds" (`KismetMathLibrary.Conv_VectorToLinearColor` (`SceneComponent.K2_GetComponentScale` _box)))
  (`KismetMaterialLibrary.SetVectorParameterValue` "/Game/Blueprints/DissolveByObject/MPC_Box_Data.MPC_Box_Data" "X" (`KismetMathLibrary.Conv_VectorToLinearColor` (`SceneComponent.GetForwardVector` _box_2)))
  (`KismetMaterialLibrary.SetVectorParameterValue` "/Game/Blueprints/DissolveByObject/MPC_Box_Data.MPC_Box_Data" "Y" (`KismetMathLibrary.Conv_VectorToLinearColor` (`SceneComponent.GetRightVector` _box_2)))
  (`KismetMaterialLibrary.SetVectorParameterValue` "/Game/Blueprints/DissolveByObject/MPC_Box_Data.MPC_Box_Data" "Z" (`KismetMathLibrary.Conv_VectorToLinearColor` (`SceneComponent.GetUpVector` _box_2))))