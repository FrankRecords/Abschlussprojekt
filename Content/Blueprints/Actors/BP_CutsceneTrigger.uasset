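; Trigger actor that plays a media cutscene in an overlay widget on overlap, disabling player character input meanwhile.
; A DoOnce gates playback, and reaching the video's end removes the overlay, restores input and re-arms the trigger if Retriggerable.
; Holding the skip action runs a timeline that fills the overlay's slider, then closes the video and restores input.
; Releasing early stops and zeroes the slider.
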(event `self.ReceiveBeginPlay`
  (add `MediaPlayer.OnEndReached` (`self.MediaPlayer`) (delegate `CloseVideo`)))

(event `CloseVideo`
  (bind _returnvalue (`GameplayStatics.GetPlayerController` 0))
  (bind _cutscenewidget (`self.CutsceneWidget`)
    (:`then`
      (`Widget.RemoveFromParent` _cutscenewidget)
      (`self.EnableInput` (`GameplayStatics.GetPlayerCharacter` 0) (`GameplayStatics.GetPlayerController` 0))
      (if (`self.Retriggerable`)
        (goto _label :!via `Reset`)))
    (:`else`)))

(event `self.CutsceneTrigger.OnComponentBeginOverlap`
  (params (OverlappedComponent :type "PrimitiveComponent Object Reference") (OtherActor :type "Actor Object Reference") (OtherComp :type "PrimitiveComponent Object Reference") (OtherBodyIndex :type Integer) (bFromSweep :type Boolean) (SweepResult :type "HitResult Structure (by ref)"))
  (bind _returnvalue (`GameplayStatics.GetPlayerController` 0))
  (`/Engine/EditorBlueprintResources/StandardMacros.DoOnce` false :!label _label
    (:`Completed`
      (`self.CutsceneWidget`
        (:`then`
          _)
        (:`else`
          (bind _returnvalue_2 (`|CreateWidget` "/Game/CommonUI/MainWidgets/UI_CutsceneOverlay.UI_CutsceneOverlay_C" (`GameplayStatics.GetPlayerController` 0)))
          (set `self.CutsceneWidget` _returnvalue_2)))
      (`UserWidget.AddToViewport` (`self.CutsceneWidget`) 0)
      (`MediaPlayer.OpenSource` (`self.MediaPlayer`) (`self.SourceToPlay`))
      (`self.EnableInput` _returnvalue)
      (`self.DisableInput` (`GameplayStatics.GetPlayerCharacter` 0) _returnvalue))))

(event `EnhancedInput|/Game/CommonUI/Input/EnhancedInput/Actions/IA_UI_SkipCutscene`
  (params (ActionValue :type Boolean) (ElapsedSeconds :type "Float (double-precision)") (TriggeredSeconds :type "Float (double-precision)") (InputAction :type "InputAction Object Reference" :default "/Game/CommonUI/Input/EnhancedInput/Actions/IA_UI_SkipCutscene.IA_UI_SkipCutscene"))
  (bind _cutscenewidget (`self.CutsceneWidget`))
  (:`Triggered`
    (if (`Widget.IsInViewport` (`self.CutsceneWidget`))
      (bind (_direction _time) (`Timeline|SliderTimeline` :!via `PlayFromStart` :!label _label_2)
        (:`Update`
          (`/Game/CommonUI/MainWidgets/UI_CutsceneOverlay.UpdateSliderValue` _cutscenewidget _time))
        (:`Finished`
          (`Widget.RemoveFromParent` _cutscenewidget)
          (`MediaPlayer.Close` (`self.MediaPlayer`))
          (`self.EnableInput` (`GameplayStatics.GetPlayerCharacter` 0) (`GameplayStatics.GetPlayerController` 0))))))
  (:`Completed`
    (`|ExecutionSequence`
      (:`then_0`
        (goto _label_2 :!via `Stop`))
      (:`then_1`
        (`/Game/CommonUI/MainWidgets/UI_CutsceneOverlay.UpdateSliderValue` (`self.CutsceneWidget`) 0.0)))))

(fn `UserConstructionScript`)