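; Car actor that drives along a referenced path spline from start to end.
; On BeginPlay it starts the movement and plays a wheel-spin animation on its mesh, looped according to a flag.
; A timeline maps its Move value to distance along the spline and teleports the actor to that world location and rotation.
; When the timeline finishes it only clears the loop flag, without stopping or replaying the animation.
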(event `self.ReceiveBeginPlay`
  (`self.StartMoving`)
  (`SkeletalMeshComponent.PlayAnimation` (`self.Mesh`) "/Game/Blueprints/CarBPs/Anims/Anim_WheelSpin.Anim_WheelSpin" (`self.ShoudLoop?`)))

(event `StartMoving`
  (bind (_direction _move) (`Timeline|Timeline`)
    (:`Update`
      (bind (_returnvalue_location _returnvalue_rotation) (`KismetMathLibrary.BreakTransform` (`SplineComponent.GetTransformAtDistanceAlongSpline` (`/Game/Blueprints/RoadBPs/BP_SplineRoads.Spline` (`self.PathSpline`)) (`KismetMathLibrary.Lerp` 0.0 (`SplineComponent.GetSplineLength` (`/Game/Blueprints/RoadBPs/BP_SplineRoads.Spline` (`self.PathSpline`))) _move) "World" false)))
      (`self.K2_SetActorLocationAndRotation` _returnvalue_location _returnvalue_rotation false true))
    (:`Finished`
      (set `self.ShoudLoop?` false))))

(fn `UserConstructionScript`)