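; BP_HighGrass is a high grass obstacle that shrinks away the first time a BP_Snail enters its trigger box.
; A DoOnce, never reset here, starts two timelines together that drive the uniform world scale of the HighGrass and HighGrass21 components.
; When the HighGrass timeline finishes, collision is disabled on HighGrass and the BlockCharakter blocker.
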(event `self.Box.OnComponentBeginOverlap`
  (params (OverlappedComponent :type "PrimitiveComponent Object Reference") (OtherActor :type "Actor Object Reference") (OtherComp :type "PrimitiveComponent Object Reference") (OtherBodyIndex :type Integer) (bFromSweep :type Boolean) (SweepResult :type "HitResult Structure (by ref)"))
  (bind _highgrass (`self.HighGrass`))
  (cast `/Game/Characters/NPC/Snail/BP_Snail` OtherActor)
  (`/Engine/EditorBlueprintResources/StandardMacros.DoOnce` false
    (:`Completed`
      (`|ExecutionSequence`
        (:`then_0`
          (bind (_direction _shrink) (`Timeline|ShrinkGrass`)
            (:`Update`
              (`SceneComponent.SetWorldScale3D` _highgrass (`KismetMathLibrary.MakeVector` _shrink _shrink _shrink)))
            (:`Finished`
              (`PrimitiveComponent.SetCollisionEnabled` _highgrass "NoCollision")
              (`PrimitiveComponent.SetCollisionEnabled` (`self.BlockCharakter`) "NoCollision"))))
        (:`then_1`
          (bind (_direction_2 _shrink_2) (`Timeline|Timeline`)
            (:`Update`
              (`SceneComponent.SetWorldScale3D` (`self.HighGrass21`) (`KismetMathLibrary.MakeVector` _shrink_2 _shrink_2 _shrink_2)))))))))

(fn `UserConstructionScript`)