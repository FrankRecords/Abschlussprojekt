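; BP_OpenableDoor is an interactable door actor that toggles open and closed, or plays a locked sound when opening is not allowed.
; An Interaction event flips the Open state and plays or reverses a timeline that lerps the door's relative rotation between start and end rotations.
; A trigger box shows or hides an interaction widget when an actor tagged Player enters or leaves it.
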(event `OpenDoor`
  (bind (_direction _doormovement) (`Timeline|OpenCloseDoor` :!label _label)
    (:`Update`
      (`SceneComponent.K2_SetRelativeRotation` (`self.DoorActor`) (`KismetMathLibrary.RLerp` (`self.StartRotation`) (`self.EndRotation`) _doormovement) false false))))

(event `CloseDoor`
  (goto _label :!via `Reverse`))

(event `self.WidgetBox.OnComponentBeginOverlap`
  (params (OverlappedComponent :type "PrimitiveComponent Object Reference") (OtherActor :type "Actor Object Reference") (OtherComp :type "PrimitiveComponent Object Reference") (OtherBodyIndex :type Integer) (bFromSweep :type Boolean) (SweepResult :type "HitResult Structure (by ref)"))
  (if (`self.ActorHasTag` OtherActor "Player")
    (`SceneComponent.SetVisibility` (`self.InteractWidget`) true false)))

(event `self.WidgetBox.OnComponentEndOverlap`
  (params (OverlappedComponent :type "PrimitiveComponent Object Reference") (OtherActor :type "Actor Object Reference") (OtherComp :type "PrimitiveComponent Object Reference") (OtherBodyIndex :type Integer))
  (if (`self.ActorHasTag` OtherActor "Player")
    (`SceneComponent.SetVisibility` (`self.InteractWidget`) false false)))

(event `/Game/Blueprints/Interfaces/BPI_Interact.Interaction`
  (params (CharacterRef :type "/Game/Characters/ThirdPerson/Blueprints/BP_ThirdPersonCharacter Object Reference"))
  (if (`self.AllowOpening?`)
    (if (`self.Open?`)
      (`self.CloseDoor`)
      (set `self.Open?` false)
      (else
        (`self.OpenDoor`)
        (bind _output_get (set `self.Open?` true))
        (`KismetSystemLibrary.PrintString` (`KismetStringLibrary.Conv_BoolToString` _output_get))))
    (else
      (`GameplayStatics.PlaySoundAtLocation` "/Game/Sound/SFX/Door/DoorLocked.DoorLocked" (`self.K2_GetActorLocation`) (struct) 1.0 1.0 0.0 "/Game/Sound/DefaultAttenuation.DefaultAttenuation" null null null))))

(fn `UserConstructionScript`)