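; BP_DestroyKnive is an interactable spot where the player gives up the knife.
; A trigger box shows the interact widget while a tagged player carrying the knife overlaps it.
; Interaction unequips the knife and removes it from the character's inventory.
; A successful removal reports the "kniveopen" objective through the cached player reference, plays a drop sound, flags the knife as tried and plays a delayed 2D sound.
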(event `self.ReceiveBeginPlay`
  (bind _asbp_third_person_character (cast `/Game/Characters/ThirdPerson/Blueprints/BP_ThirdPersonCharacter` (`GameplayStatics.GetPlayerCharacter` 0)))
  (set `self.PlayerRef` _asbp_third_person_character))

(event `self.TriggerBox.OnComponentBeginOverlap`
  (params (OverlappedComponent :type "PrimitiveComponent Object Reference") (OtherActor :type "Actor Object Reference") (OtherComp :type "PrimitiveComponent Object Reference") (OtherBodyIndex :type Integer) (bFromSweep :type Boolean) (SweepResult :type "HitResult Structure (by ref)"))
  (if (`self.ActorHasTag` OtherActor "Player")
    (if (`/Game/Characters/ThirdPerson/Blueprints/BP_ThirdPersonCharacter.HasKnive?` (`self.PlayerRef`))
      (`SceneComponent.SetVisibility` (`self.InteractWidget`) true false))))

(event `self.TriggerBox.OnComponentEndOverlap`
  (params (OverlappedComponent :type "PrimitiveComponent Object Reference") (OtherActor :type "Actor Object Reference") (OtherComp :type "PrimitiveComponent Object Reference") (OtherBodyIndex :type Integer))
  (if (`self.ActorHasTag` OtherActor "Player")
    (`SceneComponent.SetVisibility` (`self.InteractWidget`) false false)))

(event `/Game/Blueprints/Interfaces/BPI_Interact.Interaction`
  (params (CharacterRef :type "/Game/Characters/ThirdPerson/Blueprints/BP_ThirdPersonCharacter Object Reference"))
  (if (`/Game/Characters/ThirdPerson/Blueprints/BP_ThirdPersonCharacter.HasKnive?` CharacterRef)
    (`/Game/Characters/ThirdPerson/Blueprints/BP_ThirdPersonCharacter.UnequipItem` CharacterRef true false)
    (bind _success_ (`/Game/CommonUI/03_Inventory/BP_Inventory.RemoveItem` (`/Game/Characters/ThirdPerson/Blueprints/BP_ThirdPersonCharacter.InventoryReference` CharacterRef) "/Game/CommonUI/03_Inventory/ItemClasses/BP_EquipItem_Knive.BP_EquipItem_Knive_C" 1))
    (if _success_
      (`/Game/Characters/ThirdPerson/Blueprints/BP_ThirdPersonCharacter.OnObjectiveIDCalled` (`self.PlayerRef`) "kniveopen")
      (`GameplayStatics.PlaySoundAtLocation` "/Game/CommonUI/01_AudioUI/Inventory/BackpackDroptoUnknownSurface_MNXwO.BackpackDroptoUnknownSurface_MNXwO" (`self.K2_GetActorLocation`) (struct) 0.7 1.0 0.0 "/Game/Sound/DefaultAttenuation.DefaultAttenuation" null null null)
      (set `/Game/Characters/ThirdPerson/Blueprints/BP_ThirdPersonCharacter.TriedKnive?` true CharacterRef)
      (`KismetSystemLibrary.Delay` 1.0)
      (`GameplayStatics.PlaySound2D` "/Game/Sound/Dialogue/Friend/F-004.F-004" 0.7 1.0 0.0 null null))))

(fn `UserConstructionScript`)