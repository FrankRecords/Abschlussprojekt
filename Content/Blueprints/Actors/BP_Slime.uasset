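; BP_Slime is an interactable slime that the player collects with a glass, advancing the "pickupslime" objective.
; A trigger box shows the interact widget only while a glass-holding player overlaps it.
; On interaction it unequips the glass, swaps it in the inventory for a full slime glass, reports the objective, and plays a timeline that lerps the slime's world scale from start to end size.
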(event `self.ReceiveBeginPlay`
  (bind _asbp_third_person_character (cast `/Game/Characters/ThirdPerson/Blueprints/BP_ThirdPersonCharacter` (`GameplayStatics.GetPlayerCharacter` 0)))
  (set `self.PlayerRef` _asbp_third_person_character))

(event `self.TriggerBox.OnComponentBeginOverlap`
  (params (OverlappedComponent :type "PrimitiveComponent Object Reference") (OtherActor :type "Actor Object Reference") (OtherComp :type "PrimitiveComponent Object Reference") (OtherBodyIndex :type Integer) (bFromSweep :type Boolean) (SweepResult :type "HitResult Structure (by ref)"))
  (if (`self.ActorHasTag` OtherActor "Player")
    (if (`/Game/Characters/ThirdPerson/Blueprints/BP_ThirdPersonCharacter.HasGlass?` (`self.PlayerRef`))
      (`SceneComponent.SetVisibility` (`self.InteractWidget`) true false))))

(event `self.TriggerBox.OnComponentEndOverlap`
  (params (OverlappedComponent :type "PrimitiveComponent Object Reference") (OtherActor :type "Actor Object Reference") (OtherComp :type "PrimitiveComponent Object Reference") (OtherBodyIndex :type Integer))
  (if (`self.ActorHasTag` OtherActor "Player")
    (`SceneComponent.SetVisibility` (`self.InteractWidget`) false false)))

(event `self.Interaction`
  (params (CharacterRef :type "/Game/Characters/ThirdPerson/Blueprints/BP_ThirdPersonCharacter Object Reference"))
  (bind _inventoryreference (`/Game/Characters/ThirdPerson/Blueprints/BP_ThirdPersonCharacter.InventoryReference` CharacterRef))
  (if (`/Game/Characters/ThirdPerson/Blueprints/BP_ThirdPersonCharacter.HasGlass?` CharacterRef)
    (`/Game/Characters/ThirdPerson/Blueprints/BP_ThirdPersonCharacter.UnequipItem` CharacterRef true false)
    (bind _success_ (`/Game/CommonUI/03_Inventory/BP_Inventory.RemoveItem` _inventoryreference "/Game/CommonUI/03_Inventory/ItemClasses/BP_EquipItem_Glass.BP_EquipItem_Glass_C" 1))
    (if _success_
      (`/Game/CommonUI/03_Inventory/BP_Inventory.AddItem` _inventoryreference "/Game/CommonUI/03_Inventory/ItemClasses/BP_EquipItem_GlassWithSlimeFull.BP_EquipItem_GlassWithSlimeFull_C" 1)
      (`/Game/Characters/ThirdPerson/Blueprints/BP_ThirdPersonCharacter.OnObjectiveIDCalled` (`self.PlayerRef`) "pickupslime")
      (bind (_direction _decrease) (`Timeline|Decrease` :!via `PlayFromStart`)
        (:`Update`
          (`SceneComponent.SetWorldScale3D` (`self.Slime`) (`KismetMathLibrary.VLerp` (`self.StartSlime`) (`self.EndSlime`) _decrease)))))))

(fn `UserConstructionScript`)