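; BP_PlaceLamp is an interactable spot where the player places the fixed lamp to complete the "placelamp" objective.
; A sphere overlap shows a transparent lamp preview while the player has the lamp, hiding it on exit until CanPlaceSlime is set.
; Interaction swaps in solid materials, reveals plug, cable and spotlight, and removes the item from hand and inventory.
; It also sets the player's CanPlaceSlime flag, which keeps the placed lamp visible.
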(event `self.ReceiveBeginPlay`
  (bind _lamp (`self.Lamp`))
  (`PrimitiveComponent.SetMaterial` _lamp 0 "/Game/Assets/Lamp/M_LampSilverTransparent.M_LampSilverTransparent")
  (`PrimitiveComponent.SetMaterial` _lamp 1 "/Game/Assets/Lamp/M_BulbTransparent.M_BulbTransparent")
  (bind _asbp_third_person_character (cast `/Game/Characters/ThirdPerson/Blueprints/BP_ThirdPersonCharacter` (`GameplayStatics.GetPlayerCharacter` 0)))
  (set `self.PlayerRef` _asbp_third_person_character))

(event `self.Sphere.OnComponentBeginOverlap`
  (params (OverlappedComponent :type "PrimitiveComponent Object Reference") (OtherActor :type "Actor Object Reference") (OtherComp :type "PrimitiveComponent Object Reference") (OtherBodyIndex :type Integer) (bFromSweep :type Boolean) (SweepResult :type "HitResult Structure (by ref)"))
  (if (`self.ActorHasTag` OtherActor "Player")
    (if (`/Game/Characters/ThirdPerson/Blueprints/BP_ThirdPersonCharacter.HasLamp?` (`self.PlayerRef`))
      (`SceneComponent.SetVisibility` (`self.Lamp`) true false))))

(event `self.Sphere.OnComponentEndOverlap`
  (params (OverlappedComponent :type "PrimitiveComponent Object Reference") (OtherActor :type "Actor Object Reference") (OtherComp :type "PrimitiveComponent Object Reference") (OtherBodyIndex :type Integer))
  (if (`self.ActorHasTag` OtherActor "Player")
    (if (not (`/Game/Characters/ThirdPerson/Blueprints/BP_ThirdPersonCharacter.CanPlaceSlime?` (`self.PlayerRef`)))
      (`SceneComponent.SetVisibility` (`self.Lamp`) false false))))

(event `/Game/Blueprints/Interfaces/BPI_Interact.Interaction`
  (params (CharacterRef :type "/Game/Characters/ThirdPerson/Blueprints/BP_ThirdPersonCharacter Object Reference"))
  (bind _playerref (`self.PlayerRef`))
  (bind _lamp (`self.Lamp`))
  (if (`/Game/Characters/ThirdPerson/Blueprints/BP_ThirdPersonCharacter.HasLamp?` CharacterRef)
    (`PrimitiveComponent.SetMaterial` _lamp 0 "/Game/Assets/Lamp/M_LampSilver.M_LampSilver")
    (`PrimitiveComponent.SetMaterial` _lamp 1 "/Game/Assets/Lamp/M_Bulb.M_Bulb")
    (set `/Game/Characters/ThirdPerson/Blueprints/BP_ThirdPersonCharacter.CanPlaceSlime?` true _playerref)
    (`SceneComponent.SetVisibility` (`self.Plug`) true false)
    (`SceneComponent.SetVisibility` (`self.Lamp`) true false)
    (`SceneComponent.SetVisibility` (`self.Cable`) true false)
    (`SceneComponent.SetVisibility` (`self.SpotLight`) true false)
    (`/Game/Characters/ThirdPerson/Blueprints/BP_ThirdPersonCharacter.OnObjectiveIDCalled` _playerref "placelamp")
    (`/Game/Characters/ThirdPerson/Blueprints/BP_ThirdPersonCharacter.UnequipItem` _playerref true false)
    (`/Game/CommonUI/03_Inventory/BP_Inventory.RemoveItem` (`/Game/Characters/ThirdPerson/Blueprints/BP_ThirdPersonCharacter.InventoryReference` _playerref) "/Game/CommonUI/03_Inventory/ItemClasses/BP_EquipItem_LampFixed.BP_EquipItem_LampFixed_C" 1)))

(fn `UserConstructionScript`)