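; Trigger actor that transforms the world once when the player character overlaps its box.
; On overlap it requests a save-data load and, after a brief delay, proceeds only if TransitionTriggered is unset.
; It notifies all BPI_TransitionWorld actors, blends Ultra Dynamic Sky/Weather to clear afternoon, saves asynchronously, fades in ambient music and destroys every BP_SpawnPortal.
; SaveData writes the new weather and time, but not the triggered flag.
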(event `self.Box.OnComponentBeginOverlap`
  (params (OverlappedComponent :type "PrimitiveComponent Object Reference") (OtherActor :type "Actor Object Reference") (OtherComp :type "PrimitiveComponent Object Reference") (OtherBodyIndex :type Integer) (bFromSweep :type Boolean) (SweepResult :type "HitResult Structure (by ref)"))
  (bind _returnvalue (`GameplayStatics.GetGameInstance`))
  (bind _transition_duration__seconds_ (`self.Transition Duration (Seconds)`))
  (cast `/Game/Characters/ThirdPerson/Blueprints/BP_ThirdPersonCharacter` OtherActor)
  (message `/Game/Blueprints/SaveGame/BPI_Persistence.RequestLoad` (`GameplayStatics.GetGameInstance`) self)
  (`KismetSystemLibrary.Delay` 0.2)
  (if (not (`self.Transition Triggered?`))
    (`/Engine/EditorBlueprintResources/StandardMacros.DoOnce` false
      (:`Completed`
        (bind _outactors (`GameplayStatics.GetAllActorsWithInterface` "/Game/Blueprints/Interfaces/BPI_TransitionWorld.BPI_TransitionWorld_C"))
        (for _array_element _outactors
          (message `/Game/Blueprints/Interfaces/BPI_TransitionWorld.TransitionWorld` _array_element))
        (`|ExecutionSequence`
          (:`then_0`
            (`/Game/UltraDynamicSky/Blueprints/Functions/UltraDynamicWeather_Functions.Change Weather · 𝖴𝖣𝖶` "/Game/UltraDynamicSky/Blueprints/Weather_Effects/Weather_Presets/Clear_Skies.Clear_Skies" _transition_duration__seconds_))
          (:`then_1`
            (`/Game/UltraDynamicSky/Blueprints/Functions/UltraDynamicSky_Functions.Transition Time of Day · 𝖴𝖣𝖲` 1400.0 _transition_duration__seconds_)
            (message `/Game/Blueprints/SaveGame/BPI_Persistence.RequestSave` _returnvalue true "SaveSlot1")
            (bind _asgi_tmwr (cast `/Game/Blueprints/GI_TMWR` _returnvalue))
            (`/Game/Blueprints/GI_TMWR.PlayMusic2D` _asgi_tmwr "/Game/Sound/Music/KOSATKA_-_Nature_Ambient_Meditation.KOSATKA_-_Nature_Ambient_Meditation" 7.0 0.15 "Linear")
            (bind _outactors_2 (`GameplayStatics.GetAllActorsOfClass` "/Game/Blueprints/Actors/BP_SpawnPortal.BP_SpawnPortal_C"))
            (for _array_element_2 _outactors_2
              (`self.K2_DestroyActor` _array_element_2))))))))

(event `/Game/Blueprints/SaveGame/BPI_Saveable.SaveData`
  (params (SaveGameRef :type "/Game/Blueprints/SaveGame/BP_SaveGame Object Reference"))
  (set `/Game/Blueprints/SaveGame/BP_SaveGame.WeatherSaveData` (make `/Game/Blueprints/SaveGame/Structs/S_WeatherSaveData` 1400.0 "/Game/UltraDynamicSky/Blueprints/Weather_Effects/Weather_Presets/Clear_Skies.Clear_Skies") SaveGameRef))

(event `/Game/Blueprints/SaveGame/BPI_Saveable.LoadData`
  (params (SaveGameRef :type "/Game/Blueprints/SaveGame/BP_SaveGame Object Reference"))
  (set `self.Transition Triggered?` (`/Game/Blueprints/SaveGame/BP_SaveGame.TransitionTriggered?` SaveGameRef)))

(fn `UserConstructionScript`)