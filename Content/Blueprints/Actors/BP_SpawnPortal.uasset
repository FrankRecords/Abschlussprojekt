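; BP_SpawnPortal is a trigger actor that stages a one-time portal reveal when its collision box is overlapped.
; The first overlap plays a sound, briefly disables player movement, plays a random reaction montage and sends the overlapping actor a look-at message.
; After timed delays it activates the Niagara portal effect at SpawnLocation, then stops the montage and restores walking.
; The construction script applies CollisionTransform to the trigger box.
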(event `SpawnPortal`
  (bind _niagara (`self.Niagara`))
  (`NiagaraComponent.SetAsset` (`self.Niagara`) (`self.NiagaraAsset`) true)
  (`ActorComponent.SetActive` _niagara true false)
  (`SceneComponent.K2_SetWorldLocation` _niagara (`SceneComponent.K2_GetComponentLocation` (`self.SpawnLocation`)) false false))

(event `self.Box.OnComponentBeginOverlap`
  (params (OverlappedComponent :type "PrimitiveComponent Object Reference") (OtherActor :type "Actor Object Reference") (OtherComp :type "PrimitiveComponent Object Reference") (OtherBodyIndex :type Integer) (bFromSweep :type Boolean) (SweepResult :type "HitResult Structure (by ref)"))
  (bind _returnvalue (`GameplayStatics.GetPlayerCharacter` 0))
  (bind _charactermovement (`Character.CharacterMovement` _returnvalue))
  (`/Engine/EditorBlueprintResources/StandardMacros.DoOnce` false
    (:`Completed`
      (`GameplayStatics.PlaySoundAtLocation` (`self.SoundToPlay`) (`SceneComponent.K2_GetComponentLocation` (`self.SpawnLocation`)) (struct) 0.6 1.0 0.0 null null null null)
      (`KismetSystemLibrary.Delay` 0.5)
      (`CharacterMovementComponent.DisableMovement` _charactermovement)
      (bind _asbp_third_person_character (cast `/Game/Characters/ThirdPerson/Blueprints/BP_ThirdPersonCharacter` _returnvalue))
      (bind _output_get (set `self.AnimStore` (select `int` (`KismetMathLibrary.RandomIntegerInRange` 0 3) :`0` "/Game/Characters/Boy/Animations/Focus_Montage.Focus_Montage" :`1` "/Game/Characters/Boy/Animations/Look_Around_Montage.Look_Around_Montage" :`2` "/Game/Characters/Boy/Animations/Nervously_Look_Around_Montage.Nervously_Look_Around_Montage" :`3` "/Game/Characters/Boy/Animations/Terrified_Montage.Terrified_Montage" :!type "AnimMontage Object Reference")))
      (`Character.PlayAnimMontage` _asbp_third_person_character _output_get 1.0 "None")
      (message `/Game/Blueprints/Interfaces/BPI_LookAt.LookAt` OtherActor (`self.SpawnLocation`))
      (`KismetSystemLibrary.Delay` 1.0)
      (`self.SpawnPortal`)
      (`KismetSystemLibrary.Delay` 2.0)
      (`Character.StopAnimMontage` _asbp_third_person_character (`self.AnimStore`))
      (`CharacterMovementComponent.SetMovementMode` _charactermovement "MOVE_Walking" 0)
      (set `self.AnimStore` null))))

(fn `UserConstructionScript`
  (`SceneComponent.K2_SetRelativeTransform` (`self.Box`) (`self.CollisionTransform`) false false))