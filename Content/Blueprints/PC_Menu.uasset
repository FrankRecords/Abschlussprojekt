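; Menu pawn that shows the main menu and sets up player input for it.
; On BeginPlay it creates UI_MainMenu, focuses its Continue button with Game and UI input and a visible cursor, then adds the IAMC_Player Enhanced Input context, registering it with user settings if needed.
; Any gamepad key press sets user focus back on the Continue button, supporting controller navigation.
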(event `self.ReceiveBeginPlay`
  (bind _returnvalue (`GameplayStatics.GetPlayerController` 0))
  ;[0.05098 0.05098 0.05098] Begin Play - Add Input Mapping
  (`|ExecutionSequence`
    (:`then_0`
      (bind _returnvalue_2 (`|CreateWidget` "/Game/UI/MainMenu/UI_MainMenu.UI_MainMenu_C" _returnvalue))
      (bind _output_get (set `self.MainMenuRef` _returnvalue_2))
      (`UserWidget.AddToViewport` _output_get 0)
      (`WidgetBlueprintLibrary.SetInputMode_GameAndUIEx` _returnvalue (`/Game/UI/MainMenu/UI_MainMenu.BT_Continue` _returnvalue_2))
      (set `PlayerController.bShowMouseCursor` true _returnvalue))
    (:`then_1`
      (bind _asplayer_controller (cast `PlayerController` (`self.GetController`)))
      (bind _returnvalue_3 (pcsubsystem `EnhancedInputLocalPlayerSubsystem` _asplayer_controller))
      (`/Engine/EditorBlueprintResources/StandardMacros.IsValid` _returnvalue_3
        (:`Is Valid`
          (`EnhancedInputSubsystemInterface.AddMappingContext` _returnvalue_3 "/Game/Blueprints/EnhancedInput/IAMC_Player.IAMC_Player" 0 (struct))
          (bind _returnvalue_4 (`EnhancedInputSubsystemInterface.GetUserSettings` _returnvalue_3))
          (if (not (`EnhancedInputUserSettings.IsMappingContextRegistered` _returnvalue_4 "/Game/Blueprints/EnhancedInput/IAMC_Player.IAMC_Player"))
            (`EnhancedInputUserSettings.RegisterInputMappingContext` _returnvalue_4 "/Game/Blueprints/EnhancedInput/IAMC_Player.IAMC_Player")))))))

(event `Key|AnyKey`
  (params (Key :type "Key Structure"))
  (:`Pressed`
    (if (`KismetInputLibrary.Key_IsGamepadKey` Key)
      (`Widget.SetUserFocus` (`/Game/UI/MainMenu/UI_MainMenu.BT_Continue` (`self.MainMenuRef`)) (`GameplayStatics.GetPlayerController` 0)))))

(fn `UserConstructionScript`)