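; BP_Portal2 is a portal-pair actor that updates two scene captures every tick to fake a view through each portal.
; Two helper components move to the player camera, and each capture copies the relative location of the opposite portal's helper.
; Each capture then looks at its parent component and derives a clamped FOV from its distance, narrowing as it moves away.
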(event `self.ReceiveTick`
  (params (DeltaSeconds :type "Float (single-precision)"))
  (`self.UpdateCameras`))

(fn `UpdateCameras`
  (`SceneComponent.K2_SetWorldLocation` (`self.PSimD2`) (`PlayerCameraManager.GetCameraLocation` (`GameplayStatics.GetPlayerCameraManager` 0)) false false)
  (`SceneComponent.K2_SetWorldLocation` (`self.PSimD1`) (`PlayerCameraManager.GetCameraLocation` (`GameplayStatics.GetPlayerCameraManager` 0)) false false)
  (`self.UpdateCaptureM` (`self.PSimD2`) (`self.P1Capture`))
  (`self.UpdateCaptureM` (`self.PSimD1`) (`self.P2Capture`))
  (return))

(fn `UserConstructionScript`)