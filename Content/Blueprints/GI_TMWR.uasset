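; Game instance that centralises save/load, settings persistence and 2D music playback with fades.
; RequestSave passes all BPI_Saveable actors to BP_SaveGame, then timestamps and writes the slot, sync or async.
; RequestLoad serves individual requesters from the loaded save, using a DoOnce-gated delayed retry while it is invalid.
; Audio, graphics, gameplay and resolution settings each use their own BP_SaveGame slot, created when missing.
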(event `LoadGame`
  (params (Async :type Boolean) (SlotToLoad :type String))
  ;[1 1 1] Load Game From Slot
  (bind _returnvalue (`GameplayStatics.DoesSaveGameExist` SlotToLoad))
  (if _returnvalue
    (if Async
      (bind _savegame (`AsyncActionHandleSaveGame.AsyncLoadGameFromSlot` SlotToLoad)
        (:`Completed`
          (bind _asbp_save_game (cast `/Game/Blueprints/SaveGame/BP_SaveGame` _savegame))
          (bind _output_get (set `self.SaveGameRef` _asbp_save_game))
          (`self.GameLoaded` _output_get)))
      (else
        (bind _returnvalue_2 (`GameplayStatics.LoadGameFromSlot` SlotToLoad))
        (bind _asbp_save_game_2 (cast `/Game/Blueprints/SaveGame/BP_SaveGame` _returnvalue_2))
        (bind _output_get_2 (set `self.SaveGameRef` _asbp_save_game_2))
        (`self.GameLoaded` _output_get_2)))))

(event `CreateSaveGame`
  ;[1 1 1] Create New Save Game
  (bind _returnvalue (`GameplayStatics.CreateSaveGameObject` "/Game/Blueprints/SaveGame/BP_SaveGame.BP_SaveGame_C"))
  (set `self.SaveGameRef` _returnvalue))

(event `SaveGame`
  (params (Async :type Boolean))
  ;[1 1 1] Save Game to Slot
  (`self.SaveTimeAndDateSlot`)
  (if Async
    (`AsyncActionHandleSaveGame.AsyncSaveGameToSlot` (`self.SaveGameRef`) (`self.SaveGameSlotName`)
      (:`Completed`
        (`self.GameSaved` (`self.SaveGameRef`))))
    (else
      (`GameplayStatics.SaveGameToSlot` (`self.SaveGameRef`) (`self.SaveGameSlotName`))
      (`self.GameSaved` (`self.SaveGameRef`)))))

(event `/Game/Blueprints/SaveGame/BPI_Persistence.RequestSave`
  (params (Async :type Boolean))
  ;[1 1 1] Event Request Save
  (bind _outactors (`GameplayStatics.GetAllActorsWithInterface` "/Game/Blueprints/SaveGame/BPI_Saveable.BPI_Saveable_C"))
  (`/Game/Blueprints/SaveGame/BP_SaveGame.SaveAllData` (`self.SaveGameRef`) _outactors)
  (`self.SaveGame` Async))

(event `/Game/Blueprints/SaveGame/BPI_Persistence.RequestLoad`
  (params (Requester :type "Object Object Reference"))
  (bind _savegameref (`self.SaveGameRef`))
  ;[1 1 1] Event Request Load
  (`/Engine/EditorBlueprintResources/StandardMacros.IsValid` _savegameref :!label _label
    (:`Is Valid`
      (`/Game/Blueprints/SaveGame/BP_SaveGame.LoadDataForRequester` _savegameref Requester)
      (goto _label_2 :!via `Reset`))
    (:`Is Not Valid`
      (`/Engine/EditorBlueprintResources/StandardMacros.DoOnce` false :!label _label_2
        (:`Completed`
          (`KismetSystemLibrary.Delay` 1.0)
          (goto _label))))))

(fn `FadeOutMusic2D`
  (params (FadeOutDuration :type "Float (single-precision)") (FadeVolumeLevel :type "Float (single-precision)") (FadeCurve :type "EAudioFaderCurve Enum" :default "Linear"))
  (bind _playingmusic (`self.PlayingMusic`)
    (:`then`
      (`AudioComponent.FadeOut` _playingmusic FadeOutDuration FadeVolumeLevel FadeCurve))
    (:`else`)))

(fn `LoadAudioSettings`
  (returns (MasterVolumeValue :type "Float (double-precision)") (MusicVolumeValue :type "Float (double-precision)") (DialogueVolumeValue :type "Float (double-precision)") (SFXVolumeValue :type "Float (double-precision)") (AmbientVolumeValue :type "Float (double-precision)"))
  (bind (_audiosettingssavedata_mastervolumevalue _audiosettingssavedata_musicvolumevalue _audiosettingssavedata_dialoguevolumevalue _audiosettingssavedata_sfxvolumevalue _audiosettingssavedata_ambientvolumevalue) (break `/Game/Blueprints/SaveGame/Structs/S_AudioSettings` (`/Game/Blueprints/SaveGame/BP_SaveGame.AudioSettingsSaveData` (`self.SaveGameDataAudio`))))
  (bind _returnvalue (`GameplayStatics.DoesSaveGameExist` (`self.AudioSaveSlot`)))
  (if _returnvalue
    (bind _returnvalue_2 (`GameplayStatics.LoadGameFromSlot` (`self.AudioSaveSlot`)))
    (bind _asbp_save_game (cast `/Game/Blueprints/SaveGame/BP_SaveGame` _returnvalue_2))
    (set `self.SaveGameDataAudio` _asbp_save_game)
    (else
      (bind _returnvalue_3 (`GameplayStatics.CreateSaveGameObject` "/Game/Blueprints/SaveGame/BP_SaveGame.BP_SaveGame_C"))
      (set `self.SaveGameDataAudio` _returnvalue_3)))
  (return _audiosettingssavedata_mastervolumevalue _audiosettingssavedata_musicvolumevalue _audiosettingssavedata_dialoguevolumevalue _audiosettingssavedata_sfxvolumevalue _audiosettingssavedata_ambientvolumevalue))

(fn `LoadGameplaySettings`
  (returns (`Gameplay Settings Save Data Controller Vibration on Off` :type Boolean) (`Gameplay Settings Save Data Invert Camera XAxis` :type Boolean) (`Gameplay Settings Save Data Invert Camera YAxis` :type Boolean) (`Gameplay Settings Save Data Camera Sensitivity` :type "Float (double-precision)"))
  (bind (_gameplaysettingssavedata_controllervibrationonoff _gameplaysettingssavedata_invertcameraxaxis _gameplaysettingssavedata_invertcamerayaxis _gameplaysettingssavedata_camerasensitivity) (break `/Game/Blueprints/SaveGame/Structs/S_GameplaySettings` (`/Game/Blueprints/SaveGame/BP_SaveGame.GameplaySettingsSaveData` (`self.SaveGameDataGameplay`))))
  (bind _returnvalue (`GameplayStatics.DoesSaveGameExist` (`self.GameplaySettingsSaveSlot`)))
  (if _returnvalue
    (bind _returnvalue_2 (`GameplayStatics.LoadGameFromSlot` (`self.GameplaySettingsSaveSlot`)))
    (bind _asbp_save_game (cast `/Game/Blueprints/SaveGame/BP_SaveGame` _returnvalue_2))
    (set `self.SaveGameDataGameplay` _asbp_save_game)
    (else
      (bind _returnvalue_3 (`GameplayStatics.CreateSaveGameObject` "/Game/Blueprints/SaveGame/BP_SaveGame.BP_SaveGame_C"))
      (set `self.SaveGameDataGameplay` _returnvalue_3)))
  (return _gameplaysettingssavedata_controllervibrationonoff _gameplaysettingssavedata_invertcameraxaxis _gameplaysettingssavedata_invertcamerayaxis _gameplaysettingssavedata_camerasensitivity))

(fn `LoadGraphicSettings`
  (returns (WindowedMode :type "EWindowMode Enum") (ScreenResolution :type "IntPoint Structure") (FPS :type String))
  (bind (_graphicsettingssavedata_windowedmode _graphicsettingssavedata_screenresolution _graphicsettingssavedata_fps) (break `/Game/Blueprints/SaveGame/Structs/S_GraphicSettings` (`/Game/Blueprints/SaveGame/BP_SaveGame.GraphicSettingsSaveData` (`self.SaveGameDataGraphic`))))
  (bind _returnvalue (`GameplayStatics.DoesSaveGameExist` (`self.GraphicsSaveSlot`)))
  (if _returnvalue
    (bind _returnvalue_2 (`GameplayStatics.LoadGameFromSlot` (`self.GraphicsSaveSlot`)))
    (bind _asbp_save_game (cast `/Game/Blueprints/SaveGame/BP_SaveGame` _returnvalue_2))
    (set `self.SaveGameDataGraphic` _asbp_save_game)
    (else
      (bind _returnvalue_3 (`GameplayStatics.CreateSaveGameObject` "/Game/Blueprints/SaveGame/BP_SaveGame.BP_SaveGame_C"))
      (set `self.SaveGameDataGraphic` _returnvalue_3)))
  (return _graphicsettingssavedata_windowedmode _graphicsettingssavedata_screenresolution _graphicsettingssavedata_fps))

(fn `LoadScreenResolutionSettings`
  (returns (ScreenResolutionIndexSaveData :type Integer))
  (bind _returnvalue (`GameplayStatics.DoesSaveGameExist` (`self.ScreenResSaveSlot`)))
  (if _returnvalue
    (bind _returnvalue_2 (`GameplayStatics.LoadGameFromSlot` (`self.ScreenResSaveSlot`)))
    (bind _asbp_save_game (cast `/Game/Blueprints/SaveGame/BP_SaveGame` _returnvalue_2))
    (set `self.SaveGameDataScreenRes` _asbp_save_game)
    (else
      (bind _returnvalue_3 (`GameplayStatics.CreateSaveGameObject` "/Game/Blueprints/SaveGame/BP_SaveGame.BP_SaveGame_C"))
      (set `self.SaveGameDataScreenRes` _returnvalue_3)))
  (return (`/Game/Blueprints/SaveGame/BP_SaveGame.ScreenResolutionIndexSaveData` (`self.SaveGameDataScreenRes`))))

(fn `PauseMusic2D`
  (params (SetPaused :type Boolean))
  (bind _playingmusic (`self.PlayingMusic`)
    (:`then`
      (`AudioComponent.SetPaused` _playingmusic SetPaused))
    (:`else`)))

(fn `PlayMusic2D`
  (params (Sound :type "SoundBase Object Reference") (FadeInDuration :type "Float (double-precision)" :default 1.0) (FadeVolumeLevel :type "Float (double-precision)" :default 0.3) (FadeCurve :type "EAudioFaderCurve Enum" :default "Linear"))
  (`self.PlayingMusic`
    (:`then`
      (`self.FadeOutMusic2D` 2.0 0.0 FadeCurve)
      (bind _returnvalue (`GameplayStatics.SpawnSound2D` Sound 1.0 1.0 0.0 null))
      (set `self.PlayingMusic` _returnvalue))
    (:`else`
      (bind _returnvalue_2 (`GameplayStatics.SpawnSound2D` Sound 1.0 1.0 0.0 null true))
      (`AudioComponent.FadeIn` _returnvalue_2 FadeInDuration FadeVolumeLevel 0.0 FadeCurve)
      (set `self.PlayingMusic` _returnvalue_2))))

(fn `RetrieveSaveData`
  (params (LOCALSaveSlotName :type String))
  (returns (SaveDateAndTime :type String))
  (bind _returnvalue (`GameplayStatics.DoesSaveGameExist` LOCALSaveSlotName))
  (if _returnvalue
    (bind _returnvalue_2 (`GameplayStatics.LoadGameFromSlot` (`local.LOCALSaveSlotName`)))
    (bind _asbp_save_game (cast `/Game/Blueprints/SaveGame/BP_SaveGame` _returnvalue_2))
    (return (`/Game/Blueprints/SaveGame/BP_SaveGame.SaveDateAndTime` _asbp_save_game))))

(fn `SaveAudioSettings`
  (params (MasterVolumeValue :type "Float (double-precision)") (MusicVolumeValue :type "Float (double-precision)") (DialogueVolumeValue :type "Float (double-precision)") (SFXVolumeValue :type "Float (double-precision)") (AmbientVolumeValue :type "Float (double-precision)"))
  (bind _returnvalue (`GameplayStatics.DoesSaveGameExist` (`self.AudioSaveSlot`)))
  (if _returnvalue
    (bind _returnvalue_2 (`GameplayStatics.LoadGameFromSlot` (`self.AudioSaveSlot`)))
    (bind _asbp_save_game (cast `/Game/Blueprints/SaveGame/BP_SaveGame` _returnvalue_2))
    (set `self.SaveGameDataAudio` _asbp_save_game)
    (else
      (bind _returnvalue_3 (`GameplayStatics.CreateSaveGameObject` "/Game/Blueprints/SaveGame/BP_SaveGame.BP_SaveGame_C"))
      (set `self.SaveGameDataAudio` _returnvalue_3)))
  (bind _savegamedataaudio (`self.SaveGameDataAudio`)
    (:`then`
      (set `/Game/Blueprints/SaveGame/BP_SaveGame.AudioSettingsSaveData` (make `/Game/Blueprints/SaveGame/Structs/S_AudioSettings` MasterVolumeValue MusicVolumeValue DialogueVolumeValue SFXVolumeValue AmbientVolumeValue) _savegamedataaudio)
      (`GameplayStatics.SaveGameToSlot` _savegamedataaudio (`self.AudioSaveSlot`)))
    (:`else`)))

(fn `SaveGameplaySettings`
  (params (`Gameplay Settings Save Data Controller Vibration on Off` :type Boolean) (`Gameplay Settings Save Data Invert Camera XAxis` :type Boolean) (`Gameplay Settings Save Data Invert Camera YAxis` :type Boolean) (`Gameplay Settings Save Data Camera Sensitivity` :type "Float (double-precision)"))
  (bind _returnvalue (`GameplayStatics.DoesSaveGameExist` (`self.GameplaySettingsSaveSlot`)))
  (if _returnvalue
    (bind _returnvalue_2 (`GameplayStatics.LoadGameFromSlot` (`self.GameplaySettingsSaveSlot`)))
    (bind _asbp_save_game (cast `/Game/Blueprints/SaveGame/BP_SaveGame` _returnvalue_2))
    (set `self.SaveGameDataGameplay` _asbp_save_game)
    (else
      (bind _returnvalue_3 (`GameplayStatics.CreateSaveGameObject` "/Game/Blueprints/SaveGame/BP_SaveGame.BP_SaveGame_C"))
      (set `self.SaveGameDataGameplay` _returnvalue_3)))
  (bind _savegamedatagameplay (`self.SaveGameDataGameplay`)
    (:`then`
      (set `/Game/Blueprints/SaveGame/BP_SaveGame.GameplaySettingsSaveData` (make `/Game/Blueprints/SaveGame/Structs/S_GameplaySettings` `Gameplay Settings Save Data Controller Vibration on Off` `Gameplay Settings Save Data Invert Camera XAxis` `Gameplay Settings Save Data Invert Camera YAxis` `Gameplay Settings Save Data Camera Sensitivity`) _savegamedatagameplay)
      (`GameplayStatics.SaveGameToSlot` _savegamedatagameplay (`self.GameplaySettingsSaveSlot`)))
    (:`else`)))

(fn `SaveGraphicSettings`
  (params (WindowedMode :type "EWindowMode Enum" :default "Fullscreen") (ScreenResolution :type "IntPoint Structure") (FPS :type String))
  (bind _returnvalue (`GameplayStatics.DoesSaveGameExist` (`self.GraphicsSaveSlot`)))
  (if _returnvalue
    (bind _returnvalue_2 (`GameplayStatics.LoadGameFromSlot` (`self.GraphicsSaveSlot`)))
    (bind _asbp_save_game (cast `/Game/Blueprints/SaveGame/BP_SaveGame` _returnvalue_2))
    (set `self.SaveGameDataGraphic` _asbp_save_game)
    (else
      (bind _returnvalue_3 (`GameplayStatics.CreateSaveGameObject` "/Game/Blueprints/SaveGame/BP_SaveGame.BP_SaveGame_C"))
      (set `self.SaveGameDataGraphic` _returnvalue_3)))
  (bind _savegamedatagraphic (`self.SaveGameDataGraphic`)
    (:`then`
      (set `/Game/Blueprints/SaveGame/BP_SaveGame.GraphicSettingsSaveData` (make `/Game/Blueprints/SaveGame/Structs/S_GraphicSettings` WindowedMode ScreenResolution FPS) _savegamedatagraphic)
      (`GameplayStatics.SaveGameToSlot` _savegamedatagraphic (`self.GraphicsSaveSlot`)))
    (:`else`)))

(fn `SaveScreenResolutionSettings`
  (params (ScreenResolutionIndexSaveData :type Integer))
  (bind _returnvalue (`GameplayStatics.DoesSaveGameExist` (`self.ScreenResSaveSlot`)))
  (if _returnvalue
    (bind _returnvalue_2 (`GameplayStatics.LoadGameFromSlot` (`self.ScreenResSaveSlot`)))
    (bind _asbp_save_game (cast `/Game/Blueprints/SaveGame/BP_SaveGame` _returnvalue_2))
    (set `self.SaveGameDataScreenRes` _asbp_save_game)
    (else
      (bind _returnvalue_3 (`GameplayStatics.CreateSaveGameObject` "/Game/Blueprints/SaveGame/BP_SaveGame.BP_SaveGame_C"))
      (set `self.SaveGameDataScreenRes` _returnvalue_3)))
  (bind _savegamedatascreenres (`self.SaveGameDataScreenRes`)
    (:`then`
      (set `/Game/Blueprints/SaveGame/BP_SaveGame.ScreenResolutionIndexSaveData` ScreenResolutionIndexSaveData _savegamedatascreenres)
      (`GameplayStatics.SaveGameToSlot` _savegamedatascreenres (`self.ScreenResSaveSlot`)))
    (:`else`)))

(fn `SaveTimeAndDateSlot`
  (bind (_returnvalue_year _returnvalue_month _returnvalue_day _returnvalue_hour _returnvalue_minute) (`KismetMathLibrary.BreakDateTime` (`KismetMathLibrary.Now`)))
  (set `/Game/Blueprints/SaveGame/BP_SaveGame.SaveDateAndTime` (`KismetStringLibrary.Concat_StrStr` "Saved at: " (`KismetStringLibrary.Conv_IntToString` _returnvalue_month) "/" (`KismetStringLibrary.Conv_IntToString` _returnvalue_day) "/" (`KismetStringLibrary.Conv_IntToString` _returnvalue_year) " at " (`KismetStringLibrary.Conv_IntToString` _returnvalue_hour) ":" (`KismetStringLibrary.Conv_IntToString` _returnvalue_minute)) (`self.SaveGameRef`)))