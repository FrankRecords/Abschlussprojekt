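; AI traffic car on Chaos vehicle physics that follows road splines and picks random next roads at their ends.
; BeginPlay runs a Timeline teleporting it along the spline, while Tick applies full throttle.
; Helper functions, not called from this event graph, steer toward a tangent look-ahead point and set throttle from target speed.
; A forward box trace flags oncoming cars to avoid; ReduceVelocity handles queued cars and traffic lights.
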(event `self.ReceiveBeginPlay`
  (bind (_direction _move) (`Timeline|Timeline`)
    (:`Update`
      (bind (_returnvalue_location _returnvalue_rotation) (`KismetMathLibrary.BreakTransform` (`SplineComponent.GetTransformAtDistanceAlongSpline` (`/Game/Blueprints/RoadBPs/BP_SplineRoads.Spline` (`self.Road`)) (`KismetMathLibrary.Lerp` 0.0 (`SplineComponent.GetSplineLength` (`/Game/Blueprints/RoadBPs/BP_SplineRoads.Spline` (`self.Road`))) _move) "World" false)))
      (`self.K2_SetActorLocationAndRotation` _returnvalue_location _returnvalue_rotation false true))))

(event `self.ReceiveTick`
  (params (DeltaSeconds :type "Float (single-precision)"))
  ;[0 1 0.01871] Tick Drive Car
  (`ChaosVehicleMovementComponent.SetThrottleInput` (`self.VehicleMovementComponent`) 1.0))

(event `/Game/Blueprints/RoadBPs/BPI_CarTrafficAI_System.SetRoad`
  (params (Road :type "/Game/Blueprints/RoadBPs/BP_SplineRoads Object Reference"))
  ;[0 0.1402 1] Movement Car
  (set `self.Road` Road))

(event `/Game/Blueprints/RoadBPs/BPI_CarTrafficAI_System.StartMoveCar`
  (params (TrafficLight :type Boolean))
  ;[0 0.1402 1] Movement Car
  (bind _output_get (set `self.ShouldStand` false))
  (`ChaosVehicleMovementComponent.SetHandbrakeInput` (`self.VehicleMovementComponent`) _output_get)
  (`self.CarMovement` true))

(event `/Game/Blueprints/RoadBPs/BPI_CarTrafficAI_System.StopCar`
  (params (TrafficLight :type Boolean))
  ;[0 0.1402 1] Movement Car
  (`self.CarMovement` false)
  (bind _output_get (set `self.ShouldStand` true))
  (`ChaosVehicleMovementComponent.SetHandbrakeInput` (`self.VehicleMovementComponent`) _output_get))

(event `CarMovement`
  (params (`Active?` :type Boolean))
  (bind _vehiclemovementcomponent (`self.VehicleMovementComponent`))
  ;[0 0.1402 1] Movement Car
  (if `Active?`
    (`ChaosVehicleMovementComponent.SetThrottleInput` _vehiclemovementcomponent 0.0)
    (`ChaosVehicleMovementComponent.SetBrakeInput` _vehiclemovementcomponent 0.0)
    (`ChaosVehicleMovementComponent.SetSteeringInput` _vehiclemovementcomponent 0.0)
    (else
      (`ChaosVehicleMovementComponent.SetBrakeInput` _vehiclemovementcomponent (* -1.0 -1.0))
      (`ChaosVehicleMovementComponent.SetThrottleInput` _vehiclemovementcomponent 0.0)
      (`ChaosVehicleMovementComponent.SetSteeringInput` _vehiclemovementcomponent 0.0))))

(fn `CheckCollision`
  (bind _arrow (`self.Arrow`))
  (bind _returnvalue (`SceneComponent.K2_GetComponentLocation` _arrow))
  (bind _outhit (`KismetSystemLibrary.BoxTraceSingle` _returnvalue (+ _returnvalue (* (`SceneComponent.GetForwardVector` _arrow) (`self.DistanceCheckCollision`))) (10.0 100.0 10.0) (`SceneComponent.K2_GetComponentRotation` _arrow) "TraceTypeQuery3" false (`|MakeArray` self :!type "Actor Object Reference") "None" true (struct :`R` 1.0 :`A` 1.0) (struct :`G` 1.0 :`A` 1.0) 1.0))
  (bind (_bblockinghit _binitialoverlap _time _distance _location _impactpoint _normal _impactnormal _physmat _hitactor) (`GameplayStatics.BreakHitResult` _outhit))
  (if _bblockinghit
    (bind _asbp_ai_car (cast `/Game/Blueprints/CarBPs/BP_AI-Car` _hitactor))
    (if (< (`KismetMathLibrary.Dot_VectorVector` (`SceneComponent.GetForwardVector` (`self.Arrow`)) (`SceneComponent.GetForwardVector` (`/Game/Blueprints/CarBPs/BP_AI-Car.Arrow` _asbp_ai_car))) -0.7)
      (set `self.AvoidCarInFront?` true)
      (else
        (`self.ReduceVelocity` _distance _hitactor)
        (set `self.AvoidCarInFront?` false)))
    (else
      (set `self.SpeedChangeRoad` (`/Game/Blueprints/RoadBPs/BP_SplineRoads.SpeedLimit` (`self.Road`)))
      (set `self.AvoidCarInFront?` false)
      (set `self.ShouldReverse?` false)
      (`self.StartMoveCar` false))))

(fn `CheckEndRoad`
  (returns (ReturnValue :type Boolean))
  (bind _road (`self.Road`)
    (:`then`
      (bind _spline (`/Game/Blueprints/RoadBPs/BP_SplineRoads.Spline` _road))
      (bind _returnvalue_x (`KismetMathLibrary.BreakVector` (`SplineComponent.FindLocationClosestToWorldLocation` _spline (`SceneComponent.K2_GetComponentLocation` (`self.Mesh`)) "World")))
      (bind _returnvalue_x_2 (`KismetMathLibrary.BreakVector` (`SplineComponent.GetLocationAtSplinePoint` _spline (`SplineComponent.GetNumberOfSplinePoints` _spline) "World")))
      (return (== _returnvalue_x _returnvalue_x_2)))
    (:`else`)))

(fn `CheckEndRoadToReduceSpeed`
  (bind _road (`self.Road`)
    (:`then`
      (if (`self.ShouldStand`)
        (set `self.ReduceSpeedChangeRoad?` false)
        (else
          (bind _spline (`/Game/Blueprints/RoadBPs/BP_SplineRoads.Spline` _road))
          (set `self.ReduceSpeedChangeRoad?` (== (`SplineComponent.GetDistanceAlongSplineAtSplineInputKey` _spline (`SplineComponent.FindInputKeyClosestToWorldLocation` _spline (`self.K2_GetActorLocation`))) 0.0)))))
    (:`else`)))

(fn `GetDrivingState`
  (returns (Throttle :type "Float (single-precision)") (Brake :type "Float (single-precision)") (Steering :type "Float (single-precision)") (HandbrakeOn :type Boolean) (ForwardSpeed :type "Float (single-precision)") (RPM :type "Float (single-precision)") (Gear :type Integer) (Automatic :type Boolean) (AllWheelsOnGround :type Boolean) (NoWheelsOnGround :type Boolean))
  (bind _vehiclemovementcomponent (`self.VehicleMovementComponent`))
  (bind _returnvalue (`ChaosVehicleMovementComponent.GetThrottleInput` _vehiclemovementcomponent))
  (bind _returnvalue_2 (`ChaosVehicleMovementComponent.GetBrakeInput` _vehiclemovementcomponent))
  (bind _returnvalue_3 (`ChaosVehicleMovementComponent.GetSteeringInput` _vehiclemovementcomponent))
  (bind _aschaos_wheeled_vehicle_movement_component (cast `ChaosWheeledVehicleMovementComponent` _vehiclemovementcomponent))
  (bind _value (`self.NumWheelsOnGround`))
  (return _returnvalue _returnvalue_2 _returnvalue_3 (`ChaosVehicleMovementComponent.GetHandbrakeInput` _vehiclemovementcomponent) (`ChaosVehicleMovementComponent.GetForwardSpeed` _vehiclemovementcomponent) (`ChaosWheeledVehicleMovementComponent.GetEngineMaxRotationSpeed` _aschaos_wheeled_vehicle_movement_component) (`ChaosVehicleMovementComponent.GetCurrentGear` _vehiclemovementcomponent) (`ChaosVehicleMovementComponent.GetUseAutoGears` _vehiclemovementcomponent) (== _value (`ChaosWheeledVehicleMovementComponent.GetNumWheels` _aschaos_wheeled_vehicle_movement_component)) (== _value 0)))

(fn `GetPath`
  (bind _returnvalue (`self.K2_GetActorLocation`))
  (bind _spline (`/Game/Blueprints/RoadBPs/BP_SplineRoads.Spline` (`self.Road`)))
  (bind _road (`self.Road`)
    (:`then`
      (if (`self.RoadNext`)
        (bind _spline_2 (`/Game/Blueprints/RoadBPs/BP_SplineRoads.Spline` _road))
        (bind (_returnvalue_roll _returnvalue_pitch _returnvalue_yaw) (`KismetMathLibrary.BreakRotator` (`KismetMathLibrary.NormalizedDeltaRotator` (`KismetMathLibrary.FindLookAtRotation` (`self.K2_GetActorLocation`) (`SplineComponent.GetLocationAtSplinePoint` _spline_2 0 "World")) (`self.K2_GetActorRotation`))))
        (set `self.DistanceSpline` (`KismetMathLibrary.MapRangeClamped` _returnvalue_yaw 20.0 -20.0 1.0 -1.0))
        (if (== (`SplineComponent.GetDistanceAlongSplineAtSplineInputKey` _spline (`SplineComponent.FindInputKeyClosestToWorldLocation` _spline (`self.K2_GetActorLocation`))) 0.0)
          (set `self.RoadNext` false)
          (else
            (`ChaosVehicleMovementComponent.SetSteeringInput` (`self.VehicleMovementComponent`) (`self.DistanceSpline`))
            (return)))
        (else
          (bind (_returnvalue_roll_2 _returnvalue_pitch_2 _returnvalue_yaw_2) (`KismetMathLibrary.BreakRotator` (`KismetMathLibrary.NormalizedDeltaRotator` (`KismetMathLibrary.FindLookAtRotation` (`self.K2_GetActorLocation`) (`SplineComponent.FindLocationClosestToWorldLocation` _spline_2 (+ (* (`KismetMathLibrary.Normal` (`SplineComponent.FindTangentClosestToWorldLocation` _spline_2 _returnvalue "World")) 500.0) _returnvalue) "World")) (`self.K2_GetActorRotation`))))
          (set `self.DistanceSpline` (`KismetMathLibrary.MapRangeClamped` _returnvalue_yaw_2 20.0 -20.0 1.0 -1.0))
          (bind _returnvalue_2 (`self.CheckEndRoad`))
          (if _returnvalue_2
            (`self.NextRoad`)
            (else
              (`ChaosVehicleMovementComponent.SetSteeringInput` (`self.VehicleMovementComponent`) (`self.DistanceSpline`))
              (return))))))
    (:`else`)))

(fn `NextRoad`
  (bind _nextroadspline (`/Game/Blueprints/RoadBPs/BP_SplineRoads.NextRoadSpline` (`self.Road`)))
  (bind _output (`|GetArrayItem` _nextroadspline (`KismetMathLibrary.RandomIntegerInRange` 0 (- (`KismetArrayLibrary.Array_Length` _nextroadspline) 1))))
  (`/Engine/EditorBlueprintResources/StandardMacros.IsValid` _output
    (:`Is Valid`
      (`/Game/Blueprints/RoadBPs/BP_SplineRoads.RemoveCarOldSpline` (`self.Road`) self)
      (bind _output_get (set `self.Road` _output))
      (`/Game/Blueprints/RoadBPs/BP_SplineRoads.AddCarCurrentSpline` _output_get self)
      (set `self.RoadNext` true))
    (:`Is Not Valid`
      (if (`/Game/Blueprints/RoadBPs/BP_SplineRoads.Remove car end Road` (`self.Road`))
        (`/Game/Blueprints/RoadBPs/BP_SplineRoads.RemoveCarOldSpline` (`self.Road`) self)
        (`self.K2_DestroyActor`)
        (else
          (`/Game/Blueprints/RoadBPs/BPI_CarTrafficAI_System.StopCar` false)
          (set `self.Road` null))))))

(fn `NumWheelsOnGround`
  (returns (Value :type Integer))
  (locals (NumWheelsOnGround :type Integer))
  (bind _aschaos_wheeled_vehicle_movement_component (cast `ChaosWheeledVehicleMovementComponent` (`self.VehicleMovementComponent`)))
  (for _index (range (`ChaosWheeledVehicleMovementComponent.GetNumWheels` _aschaos_wheeled_vehicle_movement_component))
    (if (`ChaosWheeledVehicleMovementComponent.BreakWheelStatus` (`ChaosWheeledVehicleMovementComponent.GetWheelState` _aschaos_wheeled_vehicle_movement_component _index))
      (set `local.NumWheelsOnGround` (+ (`local.NumWheelsOnGround`) 1))))
  (return (`local.NumWheelsOnGround`)))

(fn `ReduceVelocity`
  (params (Distance :type "Float (double-precision)") (Actor :type "Actor Object Reference"))
  (bind _returnvalue (< Distance 100.0))
  (cast `/Game/Blueprints/CarBPs/BP_AI-Car` Actor
    (:`then`
      (if (< Distance 250.0)
        (`self.StopCar` false)
        (else
          (set `self.SpeedChangeRoad` 5.0)
          (`/Game/Blueprints/RoadBPs/BPI_CarTrafficAI_System.StartMoveCar` false))))
    (:`CastFailed`
      (bind _asbp_traffic_light (cast `/Game/Blueprints/RoadBPs/BP_TrafficLight` Actor)
        (:`then`
          (if _returnvalue
            (if (`/Game/Blueprints/RoadBPs/BP_TrafficLight.bIsTrafficLightGreen` _asbp_traffic_light)
              (`/Game/Blueprints/RoadBPs/BPI_CarTrafficAI_System.StartMoveCar` false)
              (else
                (`self.StopCar` false)))
            (else
              (set `self.SpeedChangeRoad` 10.0))))
        (:`CastFailed`
          (bind _asbp_traffic_light_side (cast `/Game/Blueprints/RoadBPs/BP_TrafficLight_Side` Actor)
            (:`then`
              (if _returnvalue
                (if (`/Game/Blueprints/RoadBPs/BP_TrafficLight_Side.bIsTrafficLightGreen` _asbp_traffic_light_side)
                  (`/Game/Blueprints/RoadBPs/BPI_CarTrafficAI_System.StartMoveCar` false)
                  (else
                    (`self.StopCar` false)))
                (else
                  (set `self.SpeedChangeRoad` 10.0))))
            (:`CastFailed`
              (`/Game/Blueprints/RoadBPs/BPI_CarTrafficAI_System.StartMoveCar` false))))))))

(fn `SetSpeed`
  (bind _targetspeed (`self.TargetSpeed`))
  (bind _returnvalue (- _targetspeed (`ChaosVehicleMovementComponent.GetForwardSpeedMPH` (`self.VehicleMovementComponent`))))
  (if (`self.ShouldReverse?`)
    (`/Game/Blueprints/RoadBPs/BPI_CarTrafficAI_System.StopCar` false)
    (bind _vehiclemovementcomponent (`self.VehicleMovementComponent`)
      (:`then`
        (`ChaosVehicleMovementComponent.SetBrakeInput` _vehiclemovementcomponent 0.5)
        (`ChaosVehicleMovementComponent.SetSteeringInput` _vehiclemovementcomponent 1.0))
      (:`else`))
    (elif (`self.AvoidCarInFront?`)
      (bind _vehiclemovementcomponent_2 (`self.VehicleMovementComponent`)
        (:`then`
          (`ChaosVehicleMovementComponent.SetThrottleInput` _vehiclemovementcomponent_2 0.3)
          (`ChaosVehicleMovementComponent.SetSteeringInput` _vehiclemovementcomponent_2 1.0))
        (:`else`))
      (elif (`self.isTooFast`)
        (bind _vehiclemovementcomponent_3 (`self.VehicleMovementComponent`)
          (:`then`
            (`ChaosVehicleMovementComponent.SetThrottleInput` _vehiclemovementcomponent_3 (`KismetMathLibrary.MapRangeClamped` _returnvalue 0.0 50.0 0.0 1.0)))
          (:`else`))
        (else
          (set `self.TargetSpeed` (`self.SpeedChangeRoad`))
          (bind _vehiclemovementcomponent_4 (`self.VehicleMovementComponent`)
            (:`then`
              (`ChaosVehicleMovementComponent.SetThrottleInput` _vehiclemovementcomponent_4 (`KismetMathLibrary.MapRangeClamped` _returnvalue 0.0 _targetspeed 0.0 1.0)))
            (:`else`)))))))

(fn `UserConstructionScript`)