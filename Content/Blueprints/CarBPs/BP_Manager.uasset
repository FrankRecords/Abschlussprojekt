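; BP_Manager keeps the level's AI car traffic topped up to MaxCarsInScene.
; On BeginPlay it waits, longer on the tutorial map, then counts existing BP_AICar actors.
; A self-calling, delayed CheckForSpawn loop tells a random BP_CarSpawner to spawn whenever the count is below the cap, polling more slowly when full.
; The count rises with each spawn call and falls, clamped, through the CarDespawned event.
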(event `self.ReceiveTick`
  (params (DeltaSeconds :type "Float (single-precision)")))

(event `self.ReceiveBeginPlay`
  (bind _returnvalue (`GameplayStatics.GetCurrentLevelName` true))
  (if (`KismetStringLibrary.EqualEqual_StrStr` _returnvalue "L_TutorialMap")
    (`KismetSystemLibrary.Delay` 11.0)
    (else
      (`KismetSystemLibrary.Delay` 1.0)))
  (bind _outactors (`GameplayStatics.GetAllActorsOfClass` "/Game/Blueprints/CarBPs/BP_AI-Car.BP_AI-Car_C"))
  (for _ _outactors
    (bind _result (`/Engine/EditorBlueprintResources/StandardMacros.IncrementInt` (`self.CarsInScene`))
      (:`  `
        (set `self.CarsInScene` _result))))
  (`KismetSystemLibrary.Delay` 3.0)
  (`self.CheckForSpawn`))

(event `CheckForSpawn`
  (if (< (`self.CarsInScene`) (`self.MaxCarsInScene`))
    (bind _outactors (`GameplayStatics.GetAllActorsOfClass` "/Game/Blueprints/CarBPs/BP_CarSpawner.BP_CarSpawner_C"))
    (`/Game/Blueprints/CarBPs/BP_CarSpawner.SpawnCars` (`|GetArrayItem` _outactors (`KismetMathLibrary.RandomIntegerInRange` 0 (- (`KismetArrayLibrary.Array_Length` _outactors) 1))))
    (bind _result (`/Engine/EditorBlueprintResources/StandardMacros.IncrementInt` (`self.CarsInScene`))
      (:`  `
        (set `self.CarsInScene` _result)
        (`KismetSystemLibrary.Delay` 5.0)
        (`self.CheckForSpawn`)))
    (else
      (`KismetSystemLibrary.Delay` 10.0)
      (`self.CheckForSpawn`))))

(event `CarDespawned`
  (bind _result (`/Engine/EditorBlueprintResources/StandardMacros.DecrementInt` (`self.CarsInScene`))
    (:`  `
      (set `self.CarsInScene` (`KismetMathLibrary.Clamp` _result 0 35)))))

(fn `UserConstructionScript`)