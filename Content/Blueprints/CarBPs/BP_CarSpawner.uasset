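; Car spawner actor that places a randomly chosen car and puts it on the starting road.
; Each spawn picks a class at random from CarToSpawn, uses the spawner's location and scale with the Arrow component's rotation, then passes FirstRoad to the new car via SetRoad.
; BeginPlay spawns one car, and the SpawnCars event repeats the same logic for one more on each call.
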(event `self.ReceiveBeginPlay`
  (bind (_returnvalue_location _returnvalue_rotation _returnvalue_scale) (`KismetMathLibrary.BreakTransform` (`self.GetTransform`)))
  (bind _returnvalue (`|SpawnActorFromClass` (`KismetArrayLibrary.Array_Random` (`self.CarToSpawn`)) (`KismetMathLibrary.MakeTransform` _returnvalue_location (`SceneComponent.K2_GetComponentRotation` (`self.Arrow`)) _returnvalue_scale) "Undefined" "MultiplyWithRoot" null null true null))
  (`/Engine/EditorBlueprintResources/StandardMacros.IsValid` _returnvalue
    (:`Is Valid`
      (`/Game/Blueprints/RoadBPs/BPI_CarTrafficAI_System.SetRoad` _returnvalue (`self.FirstRoad`)))))

(event `SpawnCars`
  (bind (_returnvalue_location _returnvalue_rotation _returnvalue_scale) (`KismetMathLibrary.BreakTransform` (`self.GetTransform`)))
  (bind _returnvalue (`|SpawnActorFromClass` (`KismetArrayLibrary.Array_Random` (`self.CarToSpawn`)) (`KismetMathLibrary.MakeTransform` _returnvalue_location (`SceneComponent.K2_GetComponentRotation` (`self.Arrow`)) _returnvalue_scale) "Undefined" "MultiplyWithRoot" null null true null))
  (`/Engine/EditorBlueprintResources/StandardMacros.IsValid` _returnvalue
    (:`Is Valid`
      (`/Game/Blueprints/RoadBPs/BPI_CarTrafficAI_System.SetRoad` _returnvalue (`self.FirstRoad`)))))

(fn `UserConstructionScript`)